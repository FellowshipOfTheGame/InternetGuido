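; GM_Loading is a loading-screen game mode that shows the HUD_Loading widget and travels to a random next stage.
; On BeginPlay it picks a stage from BP_GuidoInstance's CurrentStages and removes a randomly indexed entry, rolled separately so possibly a different one.
; When that pool empties, it refills from Stages.
; Tick counts DelayTest down, then opens the chosen level by name.
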(event Custom|Pull%20Stage
  (bind _asbp_guido_instance (Utilities|Casting|CastToBP_GuidoInstance (Game|GetGameInstance)))
  (bind _output_get (Variables|Default|SetStage (Utilities|Array|Get(acopy) (Variables|/Game/Base/BP_GuidoInstance.BP_GuidoInstance_C|GetCurrent%20Stages _asbp_guido_instance) (Math|Random|RandomIntegerinRange 0 (- (Utilities|Array|Length (Variables|/Game/Base/BP_GuidoInstance.BP_GuidoInstance_C|GetCurrent%20Stages _asbp_guido_instance)) 1)))))
  (Utilities|Array|RemoveIndex (Variables|/Game/Base/BP_GuidoInstance.BP_GuidoInstance_C|GetCurrent%20Stages _asbp_guido_instance) (Math|Random|RandomIntegerinRange 0 (- (Utilities|Array|Length (Variables|/Game/Base/BP_GuidoInstance.BP_GuidoInstance_C|GetCurrent%20Stages _asbp_guido_instance)) 1)))
  (if (== (Utilities|Array|Length (Variables|/Game/Base/BP_GuidoInstance.BP_GuidoInstance_C|GetCurrent%20Stages _asbp_guido_instance)) 0)
    (Variables|/Game/Base/BP_GuidoInstance.BP_GuidoInstance_C|SetCurrent%20Stages _asbp_guido_instance (Variables|/Game/Base/BP_GuidoInstance.BP_GuidoInstance_C|GetStages _asbp_guido_instance)))
  (Development|PrintString (Utilities|String|Append "O proximo mapa é: " _output_get)))

(event EventBeginPlay
  (bind _returnvalue (UserInterface|CreateWidget "/Game/HUD/HUD_Loading.HUD_Loading_C"))
  (bind _output_get (Variables|Default|SetHUD%20Reference _returnvalue))
  (UserInterface|Viewport|AddtoViewport _output_get 0)
  (CallFunction|PullStage))

(event EventTick
  (params (DeltaSeconds :type Float%20%28single-precision%29))
  (bind _output_get (Variables|Default|SetDelay%20Test (- (stale _output_get) DeltaSeconds)))
  (if (<= _output_get 0.0)
    (Game|OpenLevel(byName) (Utilities|String|StringToName (Variables|Default|GetStage)))))

(fn ConstructionScript)