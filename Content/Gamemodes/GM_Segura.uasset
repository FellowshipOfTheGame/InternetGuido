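; GM_Segura is a timed game mode for a minigame played with the BP_GiovannaSegura pawn.
; It sets an eight-second limit on BeginPlay and relies on its parent class for timer expiry handling.
; When time is over and the game is not already lost, it wins and makes the pawn dance if that pawn reports green, then calls the parent handler.
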(event EventBeginPlay
  (Variables|Default|SetMax%20Time 8.0)
  (|CallParentFunction))

(event EventTick
  (params (DeltaSeconds :type Float%20%28single-precision%29))
  (|CallParentFunction DeltaSeconds))

(event EventTimeIsOver
  (if (Variables|Default|GetIsGameLost)
    _
    (else
      (bind _asbp_giovanna_segura (Utilities|Casting|CastToBP_GiovannaSegura (Game|Player|GetPlayerPawn 0))
        (:then
          (bind _inside (Default|IsGreen _asbp_giovanna_segura))
          (if _inside
            (CallFunction|Win)
            (Default|Dance _asbp_giovanna_segura)))
        (:CastFailed
          _))))
  (|CallParentFunction))

(fn ConstructionScript
  (|CallParentFunction))