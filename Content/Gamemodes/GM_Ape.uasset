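; Ape game mode for a timed minigame, described as a monkey scaring soldiers.
; BeginPlay runs the parent logic and sets the game description text.
; Tick advances the timer through UpdateTime.
; When time runs out, it calls Win unless the game is already lost, then opens the Loading level.
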(event EventBeginPlay
  (|CallParentFunction)
  (Variables|Default|SetGame%20Description "Macaco assusta os soldados"))

(event EventTick
  (params (DeltaSeconds :type Float%20%28single-precision%29))
  (CallFunction|UpdateTime))

(event EventTimeIsOver
  (if (not (Variables|Default|GetIsGameLost))
    (CallFunction|Win))
  (Game|OpenLevel(byName) "Loading"))

(fn ConstructionScript
  (|CallParentFunction))