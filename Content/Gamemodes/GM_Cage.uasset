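; GM_Cage is the cage level's game mode: it spawns two lions and a bee at random spots and tracks winning and losing.
; Lion placement retries random points against earlier picks, restarting the whole layout after ten failed attempts, and fakes depth by deriving scale and Y from height.
; DecreaseLions declares a win and spawns BP_Sol when the lion count reaches zero, while Lose flags and prints defeat.
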(event Custom|Lose
  (Variables|Default|SetLost true)
  (Variables|Default|SetWon false)
  (Development|PrintString "You lost!"))

(event Custom|Create%20lions
  (while (Variables|Default|GetFail)
    (Variables|Default|SetFail false)
    (Utilities|FlowControl|ForLoopwithBreak 1 (Variables|Default|GetLeaos) :!label _label
      (:LoopBody
        (bind (_coordinates _scale _rotation _erro) (CallFunction|RandomCoordinates (Variables|Default|GetLionCooordinates)))
        (if _erro
          (Utilities|Array|Clear (Variables|Default|GetLionCooordinates))
          (Utilities|Array|Clear (Variables|Default|GetLionScale))
          (Utilities|Array|Clear (Variables|Default|GetLionRotation))
          (Variables|Default|SetFail true)
          (goto _label Break)
          (else
            (Utilities|Array|Add (Variables|Default|GetLionCooordinates) _coordinates)
            (Utilities|Array|Add (Variables|Default|GetLionScale) _scale)
            (Utilities|Array|Add (Variables|Default|GetLionRotation) _rotation))))))
  (for _index (range 0 (- (Variables|Default|GetLeaos) 1))
    (Game|SpawnActorfromClass "/Game/Blueprints/BP_Leao.BP_Leao_C" (Math|Transform|MakeTransform (Utilities|Array|Get(acopy) (Variables|Default|GetLionCooordinates) _index) (Utilities|Array|Get(acopy) (Variables|Default|GetLionRotation) _index) (Utilities|Array|Get(acopy) (Variables|Default|GetLionScale) _index)) "Undefined" 0 0)))

(event Custom|CreateBee
  (Game|SpawnActorfromClass "/Game/Blueprints/BP_Bee.BP_Bee_C" (Math|Transform|MakeTransform (Math|Vector|MakeVector (Math|Random|RandomFloatinRange 2e+02 1.7e+03) 1e+02 (Math|Random|RandomFloatinRange 6.2e+02 1e+03)) (Math|Rotator|MakeRotator 0.0 (Math|Random|RandomFloatinRange -5.0 5.0) 0.0) "0.750000,1,0.750000") "Undefined" 0 0))

(event Custom|DecreaseLions
  (bind _result (Math|Integer|DecrementInt (Variables|Default|GetLeaos))
    (:%20%20
      (if (== _result 0)
        (Variables|Default|SetWon true)
        (Variables|Default|SetLost false)
        (Development|PrintString "YOU WON!")
        (Game|SpawnActorfromClass "/Game/Blueprints/BP_Sol.BP_Sol_C" (Math|Transform|MakeTransform "1900.000000, 0,700.000000" "0, 0, 0" "1.500000,1,1.500000") "Undefined" 0 0)))))

(event EventBeginPlay
  (|CallParentFunction)
  (Variables|Default|SetLeaos 2)
  (CallFunction|CreateLions)
  (CallFunction|CreateBee))

(fn ConstructionScript
  (|CallParentFunction))

(fn RandomCoordinates
  (params (Older :type Array%20of%20Vectors))
  (LocalVariables|SetRandonX (Math|Random|RandomFloatinRange 2e+02 1.72e+03))
  (LocalVariables|SetRandonZ (Math|Random|RandomFloatinRange 2e+02 5.4e+02))
  (while (and (LocalVariables|GetLooping) (< (LocalVariables|GetErros) 10))
    (LocalVariables|SetLooping false)
    ;[1 1 1] Checking if there are is another lion at the spot
    (bind _index (Utilities|FlowControl|ForLoopwithBreak 0 (Utilities|Array|Length Older) :!label _label)
      (:LoopBody
        (if (or (< (- (LocalVariables|GetRandonX) (.X (Math|Vector|BreakVector (Utilities|Array|Get(acopy) Older _index)))) 4e+02) (< (- (LocalVariables|GetRandonZ) (.Z (Math|Vector|BreakVector (Utilities|Array|Get(acopy) Older _index)))) 1.2e+02))
          (LocalVariables|SetLooping true)
          (LocalVariables|SetRandonX (Math|Random|RandomFloatinRange 2e+02 1.72e+03))
          (LocalVariables|SetRandonZ (Math|Random|RandomFloatinRange 2e+02 5.4e+02))
          (Math|Integer|IncrementInt (LocalVariables|GetErros)
            (:%20%20
              (goto _label Break)))))))
  (return (Math|Vector|MakeVector (LocalVariables|GetRandonX) (- 2e+02 (* (/ (LocalVariables|GetRandonZ) 5.4e+02) 2e+02)) (LocalVariables|GetRandonZ)) (Math|Vector|MakeVector (- 0.4 (* (/ (LocalVariables|GetRandonZ) 5.4e+02) 0.3)) 1.0 (- 0.4 (* (/ (LocalVariables|GetRandonZ) 5.4e+02) 0.3))) (Math|Rotator|MakeRotator 0.0 (Math|Random|RandomFloatinRange -1e+01 1e+01) 0.0) (== (LocalVariables|GetErros) 10)))