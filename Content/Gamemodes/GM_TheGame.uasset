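; GM_TheGame is the game mode for a short timed round that is lost automatically, with a Portuguese description saying someone seems to have lost.
; BeginPlay sets the time limit and description, runs the parent logic, then adds the HUD_TheGame widget to the viewport.
; Tick runs the parent update and calls Lost once, guarded by OneTime, when CurrentTime falls to half of MaxTime or below.
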(event EventBeginPlay
  (Variables|Default|SetMax%20Time 5.0)
  (Variables|Default|SetGame%20Description "É, parece que alguem perdeu...")
  (|CallParentFunction)
  (bind _returnvalue (UserInterface|CreateWidget "/Game/HUD/HUD_TheGame.HUD_TheGame_C"))
  (UserInterface|Viewport|AddtoViewport _returnvalue 0))

(event EventTick
  (params (DeltaSeconds :type Float%20%28single-precision%29))
  (|CallParentFunction DeltaSeconds)
  (if (and (<= (Variables|Default|GetCurrent%20Time) (/ (Variables|Default|GetMax%20Time) 2.0)) (Variables|Default|GetOne%20time))
    (CallFunction|Lost)
    (Variables|Default|SetOne%20time false)))

(fn ConstructionScript
  (|CallParentFunction))