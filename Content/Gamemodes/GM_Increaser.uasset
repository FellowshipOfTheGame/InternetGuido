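; GM_Increaser is a game mode for a timed transition level that shows an increaser HUD, then opens the next stage.
; On BeginPlay it pulls the next map from BP_GuidoInstance and sets the duration to a multiple of the microgame time.
; It creates HUD_Increaser, flagging whether the current level name starts with "Speed".
; Tick accumulates time and opens the pulled map once the duration elapses.
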(event EventBeginPlay
  (bind _asbp_guido_instance (Utilities|Casting|CastToBP_GuidoInstance (Game|GetGameInstance)))
  (Variables|Default|SetMaxTime (* (Variables|/Game/Base/BP_GuidoInstance.BP_GuidoInstance_C|GetMicroGame%20Time _asbp_guido_instance) 3.0))
  (bind _stage (Default|PullStage _asbp_guido_instance))
  (Variables|Default|SetNext%20Map _stage)
  (bind _returnvalue (Game|GetCurrentLevelName true))
  (bind _output_get (Variables|Default|SetIsSpeed (Utilities|String|StartsWith _returnvalue "Speed")))
  (bind _returnvalue_2 (UserInterface|CreateWidget "/Game/HUD/HUD_Increaser.HUD_Increaser_C" 0 self _output_get))
  (bind _output_get_2 (Variables|Default|SetHUD%20Reference _returnvalue_2))
  (UserInterface|Viewport|AddtoViewport _output_get_2 0))

(event EventTick
  (params (DeltaSeconds :type Float%20%28single-precision%29))
  (bind _output_get (Variables|Default|SetTime%20Counter (+ DeltaSeconds (Variables|Default|GetTime%20Counter))))
  (if (>= _output_get (Variables|Default|GetMaxTime))
    (Game|OpenLevel(byName) (Utilities|String|StringToName (Variables|Default|GetNext%20Map)))))

(fn ConstructionScript)