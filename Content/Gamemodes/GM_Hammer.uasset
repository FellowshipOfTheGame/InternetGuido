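; GM_Hammer is a game mode Blueprint, apparently for a hammer-themed game, that sets the time limit and win reaction on top of its parent class.
; On BeginPlay it sets MaxTime before calling the parent, which presumably handles the timing.
; Win runs the parent logic, then calls Dance on every entry in the Dancarinos array.
; Tick and the construction script only forward to the parent.
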(event EventWin
  (|CallParentFunction)
  (for _array_element (Variables|Default|GetDancarinos)
    (Default|Dance _array_element)))

(event EventBeginPlay
  (Variables|Default|SetMax%20Time 4.0)
  (|CallParentFunction))

(event EventTick
  (params (DeltaSeconds :type Float%20%28single-precision%29))
  (|CallParentFunction DeltaSeconds))

(fn ConstructionScript
  (|CallParentFunction))