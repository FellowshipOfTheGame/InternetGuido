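; GM_Forninho is the game mode for a short timed "Forninho" minigame that is won by removing every forninho.
; On BeginPlay it sets MaxTime to 4 seconds and takes the forninho count from the Dificulty value on BP_GuidoInstance.
; Each RetirarForninho call decrements that count and triggers Win when it reaches zero or below.
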(event Custom|Retirar%20Forninho
  (bind _result (Math|Integer|DecrementInt (Variables|Default|GetForninhos))
    (:%20%20
      (if (<= _result 0)
        (CallFunction|Win)))))

(event EventBeginPlay
  (Variables|Default|SetMax%20Time 4.0)
  (|CallParentFunction)
  (bind _asbp_guido_instance (Utilities|Casting|CastToBP_GuidoInstance (Game|GetGameInstance)))
  (Variables|Default|SetForninhos (Variables|/Game/Base/BP_GuidoInstance.BP_GuidoInstance_C|GetDificulty _asbp_guido_instance)))

(event EventTick
  (params (DeltaSeconds :type Float%20%28single-precision%29))
  (|CallParentFunction DeltaSeconds))

(fn ConstructionScript
  (|CallParentFunction))