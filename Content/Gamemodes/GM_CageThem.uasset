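; Game mode for the "Caged Lions" minigame, won by dealing with every lion within a short time limit.
; On BeginPlay it sets the description and time, then picks the lion count from the difficulty stored in BP_GuidoInstance.
; Each KilledLion call increments a counter and triggers Win when it matches that count, while Tick calls UpdateTime.
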(event Custom|Killed%20Lion
  (bind _killed_lions (Variables|Default|GetKilled%20Lions))
  (Math|Integer|IncrementInt _killed_lions
    (:%20%20
      (if (== _killed_lions (Variables|Default|GetLionsCount))
        (CallFunction|Win)))))

(event EventTick
  (params (DeltaSeconds :type Float%20%28single-precision%29))
  (CallFunction|UpdateTime))

(event EventBeginPlay
  (Variables|Default|SetGame%20Description "Caged Lions")
  (Variables|Default|SetMax%20Time 5.0)
  (|CallParentFunction)
  (bind _asbp_guido_instance (Utilities|Casting|CastToBP_GuidoInstance (Game|GetGameInstance)))
  (Variables|Default|SetLionsCount (Utilities|Select :Index (Variables|/Game/Base/BP_GuidoInstance.BP_GuidoInstance_C|GetDificulty _asbp_guido_instance) :Option%200 2 :Option%201 4 :Option%202 6 :Option%203 8)))

(fn ConstructionScript)