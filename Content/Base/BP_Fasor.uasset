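; BP_Fasor is a phasor-style oscillator that supplies a cosine-driven position value.
; Tick accumulates Degree by delta time times Frequency, so the angle advances independently of frame rate.
; GeneratePosition returns Transladation plus Amplitude times the cosine of Degree plus Phase.
; It only computes the value and does not apply it to any transform itself.
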(event EventBeginPlay)

(event EventTick
  (params (DeltaSeconds :type Float%20%28single-precision%29))
  (Variables|Default|SetDegree (+ (* DeltaSeconds (Variables|Default|GetFrequency)) (Variables|Default|GetDegree))))

(fn GeneratePosition
  (return (+ (Variables|Default|GetTransladation) (* (Variables|Default|GetAmplitude) (Math|Trig|Cos(Radians) (+ (Variables|Default|GetDegree) (Variables|Default|GetPhase)))))))