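; BP_TweenComponent is a component that animates an actor's scale along a float curve over a set duration.
; ScaleTween stores the inputs, applies the curve's starting scale, waits out the delay, sends a start message and starts a looping timer.
; Each DoScale tick samples the curve with per-axis powered time and multiplies the result by the multiplier.
; It sends update messages to the actor, then a finish message before clearing the timer.
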(event Custom|Scale%20Tween
  (params (ScaleCurve :type Curve%20Float%20Object%20Reference) (Actor :type Actor%20Object%20Reference) (Scale%20Tween :type Tween%20Data%20Structure) (Multiplier :type Vector) (Power :type Vector))
  (Variables|Scale|SetScaleCurve ScaleCurve)
  (Variables|Scale|SetScaleActor Actor)
  (Variables|Scale|SetScaleTweenData Scale%20Tween)
  (Variables|Scale|SetScaleMultiplier Multiplier)
  (Variables|Scale|SetScalePower Power)
  (Transformation|SetActorScale3D (Variables|Scale|GetScaleActor) (* (Variables|Scale|GetScaleMultiplier) (Math|Curves|GetFloatValue (Variables|Scale|GetScaleCurve) 0.0)))
  (Utilities|FlowControl|Delay (.Delay (Utilities|Struct|BreakTweenData (Variables|Scale|GetScaleTweenData))))
  (Class|TweenListener|TweenStart(Message) (Variables|Scale|GetScaleActor) (Variables|Scale|GetScaleTweenData))
  (bind _returnvalue (Utilities|Time|SetTimerbyFunctionName self "DoScale" (.Period (Utilities|CurveRateandPeriod (.Duration (Utilities|Struct|BreakTweenData (Variables|Scale|GetScaleTweenData))) (.Frequency (Utilities|Struct|BreakTweenData (Variables|Scale|GetScaleTweenData))))) true))
  (Variables|Scale|SetScaleTimeHandle _returnvalue))

(fn DoScale
  (bind _scaletweendata (Variables|Scale|GetScaleTweenData))
  (bind _scaleactor (Variables|Scale|GetScaleActor))
  (bind _scalecurve (Variables|Scale|GetScaleCurve))
  (bind _scaletweendata_2 (Variables|Scale|GetScaleTweenData))
  (bind (_duration _frequency) (Utilities|Struct|BreakTweenData _scaletweendata_2))
  (bind _output_get (Variables|Scale|SetScaleTimePassed (+ (Variables|Scale|GetScaleTimePassed) (.Curve%20Rate (Utilities|CurveRateandPeriod _duration _frequency)))))
  (Transformation|SetActorScale3D (Variables|Scale|GetScaleActor) (* (Math|Vector|MakeVector (Math|Curves|GetFloatValue _scalecurve (.x (Utilities|FloatPowerVector _output_get (Variables|Scale|GetScalePower)))) (Math|Curves|GetFloatValue _scalecurve (.y (Utilities|FloatPowerVector _output_get (Variables|Scale|GetScalePower)))) (Math|Curves|GetFloatValue _scalecurve (.z (Utilities|FloatPowerVector _output_get (Variables|Scale|GetScalePower))))) (Variables|Scale|GetScaleMultiplier)))
  (if (>= (Variables|Scale|GetScaleTimePassed) 1.0)
    (Class|TweenListener|TweenFinish(Message) _scaleactor _scaletweendata)
    (Utilities|FinishTween (Variables|Scale|GetScaleTimeHandle) (Variables|Scale|GetScaleTimePassed))
    (else
      (Class|TweenListener|TweenUpdate(Message) _scaleactor _scaletweendata (Variables|Scale|GetScaleTimePassed))))
  (return))