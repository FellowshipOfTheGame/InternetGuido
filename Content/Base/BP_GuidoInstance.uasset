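; Game instance that runs a microgame playlist, holding lives, stage count, game speed and difficulty across levels.
; InitGame resets the run and opens the first level; PullStage serves queued stages, refilled by NextStage from a shuffle bag of playable stages.
; Counters shorten microgame time and cycle difficulty, queuing announcement levels, plus a rare "TheGame" stage.
; Init loads BP_RecordTracker, which SaveGame and ClearSave update for per-playlist records.
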(event EventInit
  (bind _returnvalue (SaveGame|CreateSaveGameObject "/Game/Base/BP_RecordTracker.BP_RecordTracker_C"))
  (bind _asbp_record_tracker (Utilities|Casting|CastToBP_RecordTracker _returnvalue))
  (Variables|RecordTrackingVars|SetSaveGame _asbp_record_tracker)
  (bind _returnvalue_2 (SaveGame|LoadGamefromSlot (Variables|/Game/Base/BP_RecordTracker.BP_RecordTracker_C|GetSaveSlotName (Variables|RecordTrackingVars|GetSaveGame)) (Variables|/Game/Base/BP_RecordTracker.BP_RecordTracker_C|GetUserIndex (Variables|RecordTrackingVars|GetSaveGame))))
  (bind _asbp_record_tracker_2 (Utilities|Casting|CastToBP_RecordTracker _returnvalue_2))
  (Variables|RecordTrackingVars|SetSaveGame _asbp_record_tracker_2))

(fn NextStage
  (bind _result (Math|Integer|IncrementInt (Variables|InGameVars|GetStages%20Done))
    (:%20%20
      (if (== _result 1)
        _
        (else
          (bind (_velocityincreased _dificultyincresed) (CallFunction|UpdateTimeandDificulty))))
      ;[0.2154 0.9303 1] Add speed increase level
      (if _velocityincreased
        (Utilities|Array|Add (Variables|StageSelectionVars|GetNext%20Stages) (Utilities|String|MakeLiteralString "SpeedIncrease")))
      ;[1 0.1562 0.1562] Add dificulty increase level
      (if _dificultyincresed
        (Utilities|Array|Add (Variables|StageSelectionVars|GetNext%20Stages) (Utilities|String|MakeLiteralString "DificultyIncrease")))
      ;[0 0 0] Random chance of opening "The game" level
      (if (> (Math|Random|RandomFloat) 0.97)
        (Utilities|Array|Add (Variables|StageSelectionVars|GetNext%20Stages) (Utilities|String|MakeLiteralString "TheGame")))
      ;[1 1 1] Add a random stage from the possible ones
      (bind _number (CallFunction|PullfromArray (Variables|StageSelectionVars|GetSelectionStages)))
      (Utilities|Array|Add (Variables|StageSelectionVars|GetNext%20Stages) (Utilities|Array|Get(acopy) (Variables|StageSelectionVars|GetPlayableStages) _number)))))

(fn InitGame
  (params (LoadStages :type Array%20of%20Strings) (StagesToIncreaseSpeed :type Integer) (StagesToIncreaseDificult :type Integer) (PlaylistName :type String))
  (Variables|StageSelectionVars|SetPlayableStages LoadStages)
  (bind _output_get (Variables|InGameVars|SetIncrease%20Velocity StagesToIncreaseSpeed))
  (Variables|Counters|SetVelCounter _output_get)
  (bind _output_get_2 (Variables|InGameVars|SetIncrease%20Dificulty StagesToIncreaseDificult))
  (Variables|Counters|SetDifCounter _output_get_2)
  (Variables|RecordTrackingVars|SetCurrentPlaylist PlaylistName)
  (Variables|InGameVars|SetDificulty 1)
  (Variables|InGameVars|SetStages%20Done 0)
  (Variables|InGameVars|SetLifes 3)
  (Variables|InGameVars|SetMicroGame%20Time 1.0)
  (bind _array (CallFunction|CreateIntArray (Utilities|Array|Length (Variables|StageSelectionVars|GetPlayableStages))))
  (Variables|StageSelectionVars|SetSelectionStages _array)
  (bind _stage (CallFunction|PullStage))
  (Game|OpenLevel(byName) (Utilities|String|StringToName _stage)))

(fn CreateIntArray
  (params (Length :type Integer))
  (bind _created_array (LocalVariables|GetCreated%20Array))
  ;[1 1 1] Creates an array with numbers from 0 to n-1
  (for _index (range 0 (- Length 1))
    (Utilities|Array|Add _created_array _index))
  (return _created_array))

(fn PullfromArray
  (params (Int%20Array :type Array%20of%20Integers))
  (bind _returnvalue (Utilities|Array|Length Int%20Array))
  (if (== _returnvalue 0)
    ;[1 1 1] Creating a new Array with the same number as playable stages
    (LocalVariables|SetWasEmpty true)
    (bind _array (CallFunction|CreateIntArray (Utilities|Array|Length (Variables|StageSelectionVars|GetPlayableStages))))
    (bind _output_get (Variables|StageSelectionVars|SetSelectionStages _array))
    (bind _number (CallFunction|PullfromArray _output_get))
    (else
      (bind _output_get_2 (LocalVariables|SetReturn%20Value (Utilities|Array|Get(acopy) Int%20Array (Math|Random|RandomIntegerinRange 0 (- _returnvalue 1)))))
      (Utilities|Array|RemoveItem Int%20Array _output_get_2)))
  (return (Math|Integer|SelectInt _number (LocalVariables|GetReturn%20Value) (LocalVariables|GetWasEmpty))))

(fn UpdateTimeandDificulty
  (bind _result (Math|Integer|DecrementInt (Variables|Counters|GetVelCounter))
    (:%20%20
      (if (< _result 1)
        (Variables|InGameVars|SetMicroGame%20Time (* (Variables|InGameVars|GetMicroGame%20Time) 0.95))
        (Variables|Counters|SetVelCounter (Variables|InGameVars|GetIncrease%20Velocity))
        (LocalVariables|SetIncreaseVel true))
      (bind _result_2 (Math|Integer|DecrementInt (Variables|Counters|GetDifCounter))
        (:%20%20
          (if (< _result_2 1)
            (bind _result_3 (Math|Integer|IncrementInt (Variables|InGameVars|GetDificulty))
              (:%20%20
                (if (> _result_3 3)
                  (Variables|InGameVars|SetDificulty 1))
                (Variables|Counters|SetDifCounter (Variables|InGameVars|GetIncrease%20Dificulty))
                (LocalVariables|SetIncreaseDif true))))
          (return (LocalVariables|GetIncreaseVel) (LocalVariables|GetIncreaseDif)))))))

(fn PullStage
  (bind _next_stages (Variables|StageSelectionVars|GetNext%20Stages))
  (if (== (Utilities|Array|LastIndex (Variables|StageSelectionVars|GetNext%20Stages)) -1)
    (CallFunction|NextStage))
  (bind _output_get (LocalVariables|SetPassStage (Utilities|Array|Get(acopy) _next_stages)))
  (Utilities|Array|RemoveItem _next_stages _output_get)
  (return _output_get))

(fn SaveGame
  (params (PlayerName :type String))
  (bind _savegame (Variables|RecordTrackingVars|GetSaveGame))
  (Default|StoreRecord _savegame (Variables|RecordTrackingVars|GetCurrentPlaylist) PlayerName (Variables|InGameVars|GetStages%20Done))
  (bind _returnvalue (SaveGame|SaveGametoSlot _savegame (Variables|/Game/Base/BP_RecordTracker.BP_RecordTracker_C|GetSaveSlotName _savegame) (Variables|/Game/Base/BP_RecordTracker.BP_RecordTracker_C|GetUserIndex _savegame)))
  (return _returnvalue))

(fn ClearSave
  (bind _savegame (Variables|RecordTrackingVars|GetSaveGame))
  (Utilities|Array|Clear (Variables|/Game/Base/BP_RecordTracker.BP_RecordTracker_C|GetData _savegame))
  (bind _returnvalue (SaveGame|SaveGametoSlot _savegame (Variables|/Game/Base/BP_RecordTracker.BP_RecordTracker_C|GetSaveSlotName _savegame) (Variables|/Game/Base/BP_RecordTracker.BP_RecordTracker_C|GetUserIndex _savegame)))
  (return _returnvalue))