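; Base game mode for timed microgames, handling the HUD, countdown and win/lose results.
; On BeginPlay it shows HUD_MicroGame, scales MaxTime by the BP_GuidoInstance time multiplier, pauses the game and starts the HUD.
; Win adds a point and Lost removes a life on the game instance.
; Tick accumulates time; at the limit an undecided game counts as lost, and the HUD's EndGame follows a short delay.
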(event Custom|Initialize%20HUD%20and%20Time
  ;[1 1 1] Initialize HUD and Time
  (bind _returnvalue (UserInterface|CreateWidget "/Game/HUD/HUD_MicroGame.HUD_MicroGame_C"))
  (bind _output_get (Variables|Default|SetHUD%20Reference _returnvalue))
  (UserInterface|Viewport|AddtoViewport _output_get 0)
  (bind _asbp_guido_instance (Utilities|Casting|CastToBP_GuidoInstance (Game|GetGameInstance)))
  (Variables|Default|SetMax%20Time (* (Variables|/Game/Base/BP_GuidoInstance.BP_GuidoInstance_C|GetMicroGame%20Time _asbp_guido_instance) (Variables|Default|GetMax%20Time)))
  (Variables|Default|SetCurrent%20Time 0.0)
  (Game|SetGamePaused true)
  (Default|Start (Variables|Default|GetHUD%20Reference)))

(event Custom|Win
  ;[1 1 1] Default Control Functions
  (bind _asbp_guido_instance (Utilities|Casting|CastToBP_GuidoInstance (Game|GetGameInstance)))
  (Math|Integer|IncrementInt (Variables|/Game/Base/BP_GuidoInstance.BP_GuidoInstance_C|GetPoints _asbp_guido_instance)
    (:%20%20
      (Variables|Default|SetIsGameWon true))))

(event Custom|Lost
  ;[1 1 1] Default Control Functions
  (bind _asbp_guido_instance (Utilities|Casting|CastToBP_GuidoInstance (Game|GetGameInstance)))
  (Math|Integer|DecrementInt (Variables|/Game/Base/BP_GuidoInstance.BP_GuidoInstance_C|GetLifes _asbp_guido_instance)
    (:%20%20
      (Variables|Default|SetIsGameLost true))))

(event Custom|Time%20Is%20Over
  ;[1 1 1] Default Control Functions
  (if (Math|Boolean|NORBoolean (Variables|Default|GetIsGameWon) (Variables|Default|GetIsGameLost))
    (CallFunction|Lost))
  (Utilities|FlowControl|Delay 0.6)
  (Default|EndGame (Variables|Default|GetHUD%20Reference)))

(event EventTick
  (params (DeltaSeconds :type Float%20%28single-precision%29))
  ;[1 1 1] Default Control Functions
  (CallFunction|UpdateTime))

(event EventBeginPlay
  ;[1 1 1] Initialize HUD and Time
  (bind _returnvalue (UserInterface|CreateWidget "/Game/HUD/HUD_MicroGame.HUD_MicroGame_C"))
  (bind _output_get (Variables|Default|SetHUD%20Reference _returnvalue))
  (UserInterface|Viewport|AddtoViewport _output_get 0)
  (bind _asbp_guido_instance (Utilities|Casting|CastToBP_GuidoInstance (Game|GetGameInstance)))
  (Variables|Default|SetMax%20Time (* (Variables|/Game/Base/BP_GuidoInstance.BP_GuidoInstance_C|GetMicroGame%20Time _asbp_guido_instance) (Variables|Default|GetMax%20Time)))
  (Variables|Default|SetCurrent%20Time 0.0)
  (Game|SetGamePaused true)
  (Default|Start (Variables|Default|GetHUD%20Reference)))

(fn ConstructionScript)

(fn UpdateTime
  (bind _output_get (Variables|Default|SetCurrent%20Time (+ (Utilities|Time|GetWorldDeltaSeconds) (Variables|Default|GetCurrent%20Time))))
  (if (>= _output_get (Variables|Default|GetMax%20Time))
    (CallFunction|TimeIsOver)))