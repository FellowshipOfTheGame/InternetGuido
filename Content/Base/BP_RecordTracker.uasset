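; BP_RecordTracker keeps a top-three high score table for each playlist in an array of StageSave structs.
; GetRecord finds a playlist's entry by name, returning its index or -1.
; StoreRecord creates an entry for a new playlist, otherwise calls UpdateRecord.
; UpdateRecord appends the name and points, bubbles them upward past lower scores in parallel arrays, and trims the fourth place before writing the struct back.
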(fn GetRecord
  (params (PlaylistName :type String))
  (bind _data (Variables|DataToSave|GetData))
  (bind (_array_element _array_index) (Utilities|Array|ForEachLoopwithBreak _data :!label _label)
    (:LoopBody
      (if (Utilities|Enum|Equal(Enum) (.PlaylistName (Utilities|Struct|BreakStageSave _array_element)) PlaylistName)
        (LocalVariables|SetID%20Value _array_index)
        (goto _label Break)))
    (:Completed
      (return (select (== (LocalVariables|GetID%20Value) -1) "" (Utilities|Array|Get(acopy) _data (LocalVariables|GetID%20Value))) (LocalVariables|GetID%20Value)))))

(fn StoreRecord
  (params (PlaylistName :type String) (RecordName :type String) (RecordPoints :type Integer))
  (bind _id (CallFunction|GetRecord PlaylistName))
  (if (== _id -1)
    (Utilities|Array|Add (Variables|DataToSave|GetData) (Utilities|Struct|MakeStageSave PlaylistName (Utilities|Array|MakeArray RecordName) (Utilities|Array|MakeArray RecordPoints)))
    (else
      (CallFunction|UpdateRecord RecordName RecordPoints _id))))

(fn UpdateRecord
  (params (NewName :type String) (NewPoint :type Integer) (Index :type Integer))
  (bind _data (Variables|DataToSave|GetData))
  (bind _item (Utilities|Array|Get(acopy) _data Index))
  (bind (_playlistname _recordname _recordpoint) (Utilities|Struct|BreakStageSave _item))
  (bind _output_get (LocalVariables|SetNewNameArray _recordname))
  (Utilities|Array|Add _output_get NewName)
  (bind _output_get_2 (LocalVariables|SetNewPointArray _recordpoint))
  (Utilities|Array|Add _output_get_2 NewPoint)
  (LocalVariables|SetPlaylistName _playlistname)
  (for _index (range 0 (- (Utilities|Array|LastIndex (LocalVariables|GetNewPointArray)) 1))
    (if (> (Utilities|Array|Get(acopy) (LocalVariables|GetNewPointArray) (- (Utilities|Array|LastIndex (LocalVariables|GetNewPointArray)) _index)) (Utilities|Array|Get(acopy) (LocalVariables|GetNewPointArray) (- (- (Utilities|Array|LastIndex (LocalVariables|GetNewPointArray)) _index) 1)))
      (LocalVariables|SetPointSwitch (Utilities|Array|Get(acopy) (LocalVariables|GetNewPointArray) (- (Utilities|Array|LastIndex (LocalVariables|GetNewPointArray)) _index)))
      (LocalVariables|SetNameSwitch (Utilities|Array|Get(acopy) (LocalVariables|GetNewNameArray) (- (Utilities|Array|LastIndex (LocalVariables|GetNewPointArray)) _index)))
      (Utilities|Array|SetArrayElem (LocalVariables|GetNewPointArray) (- (Utilities|Array|LastIndex (LocalVariables|GetNewPointArray)) _index) (Utilities|Array|Get(acopy) (LocalVariables|GetNewPointArray) (- (- (Utilities|Array|LastIndex (LocalVariables|GetNewPointArray)) _index) 1)))
      (Utilities|Array|SetArrayElem (LocalVariables|GetNewNameArray) (- (Utilities|Array|LastIndex (LocalVariables|GetNewPointArray)) _index) (Utilities|Array|Get(acopy) (LocalVariables|GetNewNameArray) (- (- (Utilities|Array|LastIndex (LocalVariables|GetNewPointArray)) _index) 1)))
      (Utilities|Array|SetArrayElem (LocalVariables|GetNewPointArray) (- (- (Utilities|Array|LastIndex (LocalVariables|GetNewPointArray)) _index) 1) (LocalVariables|GetPointSwitch))
      (Utilities|Array|SetArrayElem (LocalVariables|GetNewNameArray) (- (- (Utilities|Array|LastIndex (LocalVariables|GetNewPointArray)) _index) 1) (LocalVariables|GetNameSwitch))))
  (if (== (Utilities|Array|Length (LocalVariables|GetNewPointArray)) 4)
    (Utilities|Array|RemoveIndex (LocalVariables|GetNewPointArray) 3)
    (Utilities|Array|RemoveIndex (LocalVariables|GetNewNameArray) 3))
  (Utilities|Array|SetArrayElem (Variables|DataToSave|GetData) Index (Utilities|Struct|MakeStageSave (LocalVariables|GetPlaylistName) (LocalVariables|GetNewNameArray) (LocalVariables|GetNewPointArray))))