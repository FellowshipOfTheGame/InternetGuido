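; BP_Lion is a tappable lion target that gets caged and reports to the CageThem game mode.
; On spawn it bounce-scales in through a tween component with randomized timing, playing a jump sound as the tween starts.
; The first touch on its head spawns a cage there, then removes both after a short delay and calls KilledLion.
; The construction script swaps in an alternate sprite when UseVariation is set.
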(event OnInputTouchBegin(HeadCollision)
  (params (FingerIndex :type ETouchIndex%20Enum :default "Touch1") (TouchedComponent :type Primitive%20Component%20Object%20Reference))
  (Utilities|FlowControl|DoOnce false
    (:Completed
      (Components|DestroyComponent (Variables|Default|GetHead%20Collision))
      (bind _returnvalue (Game|SpawnActorfromClass "/Game/Blueprints/BP_Cage.BP_Cage_C" (Transformation|GetWorldTransform (Variables|Default|GetHeadLocation)) "Undefined" 0 (Math|Random|RandomBool) 0))
      (Audio|PlaySound2D "/Game/Sound/SC_Hop.SC_Hop")
      (Utilities|FlowControl|Delay 0.5)
      (Actor|DestroyActor self)
      (bind _asgm_cage_them (Utilities|Casting|CastToGM_CageThem (Game|GetGameMode)))
      (Default|KilledLion _asgm_cage_them))))

(event EventTweenStart
  (Audio|PlaySound2D "/Game/Sound/Jump.Jump" 0.25 (+ 0.0 0.5)))

(event EventBeginPlay
  (Default|ScaleTween (Variables|Default|GetBP_TweenComponent) "/Game/Base/Curves/OutBounce.OutBounce" self 0.5 "1.000000,1.000000,1.000000" (Math|Vector|MakeVector (Math|Random|RandomFloatinRange 0.5 1.5) (Math|Random|RandomFloatinRange 0.5 1.5) (Math|Random|RandomFloatinRange 0.5 1.5)) (Math|Random|RandomFloatinRange 0.5 1.5) 3e+01))

(fn ConstructionScript
  (if (Variables|Default|GetUse%20Variation) ; Use variation lion?
    (Rendering|Components|Sprite|SetSprite (Variables|Default|GetLion) "/Game/Sprites/SP_Lion2.SP_Lion2")))