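; BP_Dragger is a touch-driven actor that follows the finger on the X/Z plane at fixed Y to grab, drag and flick BP_Cloud actors.
; A press picks an overlapped cloud and stores its offset, while Drag catches clouds overlapped during a hold and zeroes their velocity.
; Touch movement carries the cloud, and release sets its velocity toward the release point from the dragger, scaled by FlickVelocity.
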(event EventBeginPlay
  (Development|PrintString "Spawn"))

(event Collision|EventActorBeginOverlap
  (params (OtherActor :type Actor%20Object%20Reference))
  (CallFunction|Drag OtherActor))

(event Input|TouchEvents|InputTouch
  (params (Location :type Vector) (FingerIndex :type ETouchIndex%20Enum))
  (bind _returnvalue (Game|GetPlayerController 0))
  (bind _returnvalue_2 (Transformation|GetActorLocation))
  (bind _collider (Variables|Default|GetCollider))
  (bind _overlappingactors (Collision|GetOverlappingActors _collider 0 :!class /Script/Engine.PrimitiveComponent))
  (bind _worldlocation (Class|PlayerController|DeprojectScreenPositiontoWorld _returnvalue (.x Location) (.y Location)))
  (bind _returnvalue_3 (Math|Vector|MakeVector (.x _worldlocation) (.y _returnvalue_2) (.z _worldlocation)))
  (:Pressed
    (Transformation|SetActorLocation _returnvalue_3 false false)
    (Variables|Default|SetHolding true)
    (if (> (Utilities|Array|Length _overlappingactors) 0)
      (bind _array_element (Utilities|Array|ForEachLoopwithBreak _overlappingactors :!label _label)
        (:LoopBody
          (if (== (Utilities|GetClass _array_element) "/Game/Blueprints/BP_Cloud.BP_Cloud_C")
            (bind _output_get (Variables|Default|SetDragged _array_element))
            (Variables|Default|SetOffset (- (Transformation|GetActorLocation _output_get) (Transformation|GetActorLocation)))
            (goto _label Break))))))
  (:Released
    (bind _asbp_cloud (Utilities|Casting|CastToBP_Cloud (Variables|Default|GetDragged)))
    (Variables|/Game/Blueprints/BP_Cloud.BP_Cloud_C|SetVelocity _asbp_cloud (* (Math|Vector|Normalize (- _returnvalue_3 (Transformation|GetActorLocation))) (Variables|Default|GetFlick%20Velocity)))
    (Variables|Default|SetDragged 0)
    (Variables|Default|SetHolding false))
  (:Moved
    (Transformation|SetActorLocation _returnvalue_3 false false)
    (if (Utilities|IsValid (Variables|Default|GetDragged))
      (Transformation|SetActorLocation (Variables|Default|GetDragged) (+ _returnvalue_3 (Variables|Default|GetOffset)) false false))))

(fn ConstructionScript)

(fn Drag
  (params (ToDrag :type Actor%20Object%20Reference))
  (if (and (Variables|Default|GetHolding) (not (Utilities|IsValid (Variables|Default|GetDragged))))
    (bind _asbp_cloud (Utilities|Casting|CastToBP_Cloud ToDrag)
      (:then
        (Variables|/Game/Blueprints/BP_Cloud.BP_Cloud_C|SetVelocity _asbp_cloud "0, 0, 0")
        (Variables|Default|SetDragged _asbp_cloud)
        (Variables|Default|SetHolding false))
      (:CastFailed
        (LocalVariables|SetIsSucess false :!label _label)))
    (else
      (goto _label)))
  (return (LocalVariables|GetIsSucess)))