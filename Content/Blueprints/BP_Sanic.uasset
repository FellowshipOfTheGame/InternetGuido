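; BP_Sanic is an actor that moves along world X at Speed while spinning its Legs component, like an animated runner.
; On BeginPlay or the Starter event, it derives the leg rotation rate from MaxTime on the GM_Increaser game mode, so a shorter time means faster spinning.
; Tick applies the unswept movement and calls a helper that combines a delta-time-scaled rotation with the legs' world rotation.
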(event Custom|Starter
  (bind _asgm_increaser (Utilities|Casting|CastToGM_Increaser (Game|GetGameMode)))
  (Variables|Default|SetRotationSpeed (Math|Rotator|MakeRotator 0.0 (/ (* -3.6e+02 2e+01) (Variables|/Game/Gamemodes/GM_Increaser.GM_Increaser_C|GetMaxTime _asgm_increaser)) 0.0)))

(event EventBeginPlay
  (bind _asgm_increaser (Utilities|Casting|CastToGM_Increaser (Game|GetGameMode)))
  (Variables|Default|SetRotationSpeed (Math|Rotator|MakeRotator 0.0 (/ (* -3.6e+02 2e+01) (Variables|/Game/Gamemodes/GM_Increaser.GM_Increaser_C|GetMaxTime _asgm_increaser)) 0.0)))

(event EventTick
  (params (DeltaSeconds :type Float%20%28single-precision%29))
  (Transformation|AddActorWorldOffset (Math|Vector|MakeVector (* DeltaSeconds (Variables|Default|GetSpeed)) 0.0 0.0))
  (CallFunction|AddRotationOffset (Variables|Default|GetLegs) (Variables|Default|GetRotationSpeed)))

(fn ConstructionScript
  (Actor|Tick|SetActorTickEnabled true))

(fn AddRotationOffset
  (params (Component :type Scene%20Component%20Object%20Reference) (RotationSpeed :type Rotator))
  (Transformation|SetWorldRotation Component (Math|Rotator|CombineRotators (* RotationSpeed (Utilities|Time|GetWorldDeltaSeconds)) (Transformation|GetWorldRotation Component)) false false))