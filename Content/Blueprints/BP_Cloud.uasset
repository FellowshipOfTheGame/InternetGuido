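; BP_Cloud is a Paper2D cloud actor that drifts through the world with a randomized look.
; The Construction Script picks one of four sprites at random, then randomizes its tint, near-opaque alpha and pitch rotation.
; SetVelocity stores the drift vector, which Tick scales by delta time to offset the actor without sweep, skipping the move when velocity is near zero.
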(event EventBeginPlay)

(event Collision|EventActorBeginOverlap
  (params (OtherActor :type Actor%20Object%20Reference)))

(event EventTick
  (params (DeltaSeconds :type Float%20%28single-precision%29))
  (bind _velocity (Variables|Default|GetVelocity))
  (if (not (<= (Math|Vector|VectorLengthSquared _velocity) 0.1))
    (Transformation|AddActorWorldOffset (* _velocity DeltaSeconds))))

(fn ConstructionScript
  (bind _returnvalue (Math|Random|RandomFloatinRange 0.1 1.0))
  (Rendering|Components|Sprite|SetSprite (Variables|Default|GetPaperSprite) (Utilities|Select :Index (Math|Random|RandomIntegerinRange 0 3) :Option%200 "/Game/Sprites/SP_Cloud1.SP_Cloud1" :Option%201 "/Game/Sprites/SP_Strife.SP_Strife" :Option%202 "/Game/Sprites/SP_Cloud3.SP_Cloud3" :Option%203 "/Game/Sprites/SP_Cloud4.SP_Cloud4"))
  (Sprite|SetSpriteColor (Variables|Default|GetPaperSprite) (Math|Color|MakeColor _returnvalue _returnvalue _returnvalue (Math|Random|RandomFloatinRange 0.9 1.0)))
  (Transformation|SetRelativeRotation (Variables|Default|GetPaperSprite) (Math|Rotator|MakeRotator 0.0 (Math|Random|RandomFloatinRange 0.0 359.0) 0.0) false false))

(fn SetVelocity
  (params (NewVelocity :type Vector))
  (Variables|Default|SetVelocity NewVelocity))