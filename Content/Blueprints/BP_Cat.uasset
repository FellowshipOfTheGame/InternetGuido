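; BP_Cat is a touch minigame cat that the player feeds by dragging BP_Torrada toasts onto it.
; A Dragger component follows deprojected touches on the X/Z plane and grabs one toast via overlaps.
; Releasing it over Colision shrinks it toward the Mouth and decrements a count seeded from GameInstance difficulty.
; At zero, GM_Cat.Win fires and a delay-sequenced tween animation turns Grumpy into a flying Nyan cat with rainbow.
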(event OnComponentBeginOverlap(Dragger)
  (params (OverlappedComponent :type Primitive%20Component%20Object%20Reference) (OtherActor :type Actor%20Object%20Reference) (OtherComp :type Primitive%20Component%20Object%20Reference) (OtherBodyIndex :type Integer) (bFromSweep :type Boolean) (SweepResult :type Hit%20Result%20Structure%20%28by%20ref%29))
  (CallFunction|CanDrag OtherActor))

(event Custom|Flies%20Away
  (bind _returnvalue (Transformation|GetActorLocation))
  (bind _returnvalue_2 (Transformation|GetActorLocation))
  (bind _returnvalue_3 (Transformation|GetActorLocation))
  (bind _nyan (Variables|Default|GetNyan))
  (Rendering|SetVisibility (Variables|Default|GetGrumpy) false true)
  (Rendering|SetVisibility _nyan true false)
  (Default|ScaleTween (Variables|Default|GetBP_TweenComponent) "/Game/Curves/Linear.Linear" _nyan 0.5 "1, 1, 1" "1, 1, 1" 0.0 3e+01)
  (Utilities|FlowControl|Delay 0.5)
  (Rendering|SetVisibility (Variables|Default|GetGrumpy) false true)
  (Default|TranslationTween (Variables|Default|GetBP_TweenComponent) "/Game/Curves/Shooting.Shooting" self (- _returnvalue_2 "100.000000, 0, 0") _returnvalue_2 "NewEnumerator1" 1.0 "1,1,1" 0.0 3e+01)
  (Utilities|FlowControl|Delay 1.0)
  (Rendering|SetVisibility (Variables|Default|GetRainbow) true false)
  (Default|TranslationTween (Variables|Default|GetBP_TweenComponent) "/Game/Curves/OutBounce.OutBounce" self _returnvalue_2 (+ _returnvalue_2 "-50.000000,0.000000,300.000000") "NewEnumerator1" 1.0 "1,1,1" 0.0 3e+01)
  (Default|ScaleTween (Variables|Default|GetBP_TweenComponent) "/Game/Curves/BigSelect.BigSelect" self 1.5 "1.000000,1.000000,1.000000" "1, 1, 1" 0.0 3e+01)
  (Utilities|FlowControl|Delay 0.25)
  (Default|Vanish (Variables|Default|GetBackground))
  (Default|TranslationTween (Variables|Default|GetBP_TweenComponent) "/Game/Curves/OutBounce.OutBounce" self _returnvalue_3 (+ _returnvalue_3 "-50.000000,0.000000,-150.000000") "NewEnumerator1" 1.5 "1,1,1" 0.0 3e+01)
  (Utilities|FlowControl|Delay 1.0)
  (Default|TranslationTween (Variables|Default|GetBP_TweenComponent) "/Game/Curves/Shooting.Shooting" self (- _returnvalue "50.000000,0.000000, 0") (- _returnvalue "-50.000000, 0, 0") "NewEnumerator1" 1e+01 "1,1,1" 0.0 3e+01))

(event EventBeginPlay
  (bind _asbp_guido_instance (Utilities|Casting|CastToBP_GuidoInstance (Game|GetGameInstance)))
  (Variables|Default|SetTorradas (Variables|/Game/Base/BP_GuidoInstance.BP_GuidoInstance_C|GetDificulty _asbp_guido_instance))
  (bind _asgm_cat (Utilities|Casting|CastToGM_Cat (Game|GetGameMode)))
  (Variables|Default|SetAnimTime (* (Variables|/Game/Base/GM_MicroGame.GM_MicroGame_C|GetMax%20Time _asgm_cat) 0.5)))

(event Input|TouchEvents|InputTouch
  (params (Location :type Vector) (FingerIndex :type ETouchIndex%20Enum))
  (bind _returnvalue (Game|GetPlayerController 0))
  (bind _dragger (Variables|Default|GetDragger))
  (bind _returnvalue_2 (Transformation|GetWorldLocation _dragger))
  (bind _worldlocation (Class|PlayerController|DeprojectScreenPositiontoWorld _returnvalue (.x Location) (.y Location)))
  (bind _returnvalue_3 (Math|Vector|MakeVector (.x _worldlocation) (.y _returnvalue_2) (.z _worldlocation)))
  (:Pressed
    (Transformation|SetWorldLocation (Variables|Default|GetDragger) _returnvalue_3 false false)
    (Variables|Default|SetHolding true)
    (bind _array_element (Utilities|Array|ForEachLoopwithBreak (Collision|GetOverlappingActors (Variables|Default|GetDragger) 0 :!class /Script/Engine.PrimitiveComponent) :!label _label)
      (:LoopBody
        (if (== (Utilities|GetClass _array_element) "/Game/Blueprints/BP_Torrada.BP_Torrada_C")
          (CallFunction|CanDrag _array_element)
          (goto _label Break)))))
  (:Released
    (Variables|Default|SetHolding false)
    (bind _array_element_2 (Utilities|Array|ForEachLoopwithBreak (Collision|GetOverlappingActors (Variables|Default|GetColision) 0 :!class /Script/Engine.PrimitiveComponent) :!label _label_2)
      (:LoopBody
        (if (== _array_element_2 (Variables|Default|GetDragObject))
          (bind _asbp_torrada (Utilities|Casting|CastToBP_Torrada (Variables|Default|GetDragObject)))
          (Default|Shrink _asbp_torrada (Transformation|GetWorldLocation (Variables|Default|GetMouth)))
          (bind _result (Math|Integer|DecrementInt (Variables|Default|GetTorradas))
            (:%20%20
              (Development|PrintString (Utilities|String|ToString(Integer) _result))
              (goto _label_2 Break)))))
      (:Completed
        (Variables|Default|SetDragObject 0)
        (if (< (Variables|Default|GetTorradas) 1)
          (bind _asgm_cat (Utilities|Casting|CastToGM_Cat (Game|GetGameMode)))
          (Default|Win _asgm_cat)
          (CallFunction|FliesAway)))))
  (:Moved
    (Transformation|SetWorldLocation (Variables|Default|GetDragger) _returnvalue_3 false false)
    (if (Utilities|IsValid (Variables|Default|GetDragObject))
      (Transformation|SetActorLocation (Variables|Default|GetDragObject) _returnvalue_3 false false))))

(fn ConstructionScript)

(fn CanDrag
  (params (Object :type Actor%20Object%20Reference))
  (if (and (not (Utilities|IsValid (Variables|Default|GetDragObject))) (Variables|Default|GetHolding))
    (if (== (Utilities|GetClass Object) "/Game/Blueprints/BP_Torrada.BP_Torrada_C")
      (bind _output_get (Variables|Default|SetDragObject Object))
      (bind _asbp_torrada (Utilities|Casting|CastToBP_Torrada _output_get))
      (Default|Bounce _asbp_torrada))))