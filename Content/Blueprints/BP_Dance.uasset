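; BP_Dance is a dancer sprite actor that stays hidden until its Dance event reveals it.
; On BeginPlay it adds itself to the Dancarinos array on GM_Hammer and hides.
; Tick accumulates time and rotates the PaperSprite 180 degrees each time the Speed interval elapses, faking a two-pose dance that keeps running while hidden.
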(event Custom|Dance
  (Rendering|SetActorHiddenInGame false))

(event EventBeginPlay
  (bind _asgm_hammer (Utilities|Casting|CastToGM_Hammer (Game|GetGameMode)))
  (Utilities|Array|Add (Variables|/Game/Gamemodes/GM_Hammer.GM_Hammer_C|GetDancarinos _asgm_hammer) self)
  (Rendering|SetActorHiddenInGame true))

(event EventActorBeginOverlap
  (params (OtherActor :type Actor%20Object%20Reference)))

(event EventTick
  (params (DeltaSeconds :type Float%20%28single-precision%29))
  (bind _papersprite (Variables|Default|GetPaperSprite))
  (if (>= (+ (Variables|Default|GetCount) DeltaSeconds) (Variables|Default|GetSpeed))
    (Variables|Default|SetCount 0.0)
    (Transformation|SetWorldRotation _papersprite (Math|Rotator|CombineRotators (Transformation|GetWorldRotation _papersprite) "0.000000,180.000000, 0") false false)
    (else
      (Variables|Default|SetCount (+ (Variables|Default|GetCount) DeltaSeconds)))))

(fn ConstructionScript)