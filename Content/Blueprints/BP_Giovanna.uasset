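; Giovanna is the touch-controlled 2D character who runs sideways to catch BP_Forninho actors.
; Touch press or drag sets a world X target; Tick moves and flips the actor toward it, toggling walking and standing sprites.
; Walking limbs swing procedurally, reversing on a timer derived from GM_Forninho's MaxTime.
; Near and Nearby overlaps swap holding poses, while Colide destroys the forninho and calls RetirarForninho on the game mode.
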(event OnComponentBeginOverlap(Near)
  (params (OtherActor :type Actor%20Object%20Reference) (OtherComp :type Primitive%20Component%20Object%20Reference) (OtherBodyIndex :type Integer) (bFromSweep :type Boolean) (SweepResult :type Hit%20Result%20Structure%20%28by%20ref%29))
  (if (== (Utilities|GetClass OtherActor) "/Game/Blueprints/BP_Forninho.BP_Forninho_C")
    (CallFunction|SetRunningState false)
    (Rendering|Components|Sprite|SetSprite (Variables|Default|GetStandardSprite) "/Game/Sprites/SP_Forninho_Segurando1.SP_Forninho_Segurando1")))

(event OnComponentBeginOverlap(Nearby)
  (params (OtherActor :type Actor%20Object%20Reference) (OtherComp :type Primitive%20Component%20Object%20Reference) (OtherBodyIndex :type Integer) (bFromSweep :type Boolean) (SweepResult :type Hit%20Result%20Structure%20%28by%20ref%29))
  (if (== (Utilities|GetClass OtherActor) "/Game/Blueprints/BP_Forninho.BP_Forninho_C")
    (CallFunction|SetRunningState false)
    (Rendering|Components|Sprite|SetSprite (Variables|Default|GetStandardSprite) "/Game/Sprites/SP_Forninho_Segurando2.SP_Forninho_Segurando2")))

(event OnComponentBeginOverlap(Colide)
  (params (OtherActor :type Actor%20Object%20Reference) (OtherComp :type Primitive%20Component%20Object%20Reference) (OtherBodyIndex :type Integer) (bFromSweep :type Boolean) (SweepResult :type Hit%20Result%20Structure%20%28by%20ref%29))
  (if (== (Utilities|GetClass OtherActor) "/Game/Blueprints/BP_Forninho.BP_Forninho_C")
    (Actor|DestroyActor OtherActor)
    (bind _asgm_forninho (Utilities|Casting|CastToGM_Forninho (Game|GetGameMode)))
    (Default|RetirarForninho _asgm_forninho)
    (CallFunction|SetRunningState (Variables|Default|GetWalking))))

(event OnComponentEndOverlap(Nearby)
  (params (OtherActor :type Actor%20Object%20Reference) (OtherComp :type Primitive%20Component%20Object%20Reference) (OtherBodyIndex :type Integer))
  (if (== (Utilities|GetClass OtherActor) "/Game/Blueprints/BP_Forninho.BP_Forninho_C")
    (CallFunction|SetRunningState false)
    (Rendering|Components|Sprite|SetSprite (Variables|Default|GetStandardSprite) "/Game/Sprites/SP_Forninho_Segurando3.SP_Forninho_Segurando3")
    (CallFunction|SetRunningState (Variables|Default|GetWalking))))

(event OnComponentEndOverlap(Near)
  (params (OtherActor :type Actor%20Object%20Reference) (OtherComp :type Primitive%20Component%20Object%20Reference) (OtherBodyIndex :type Integer))
  (if (== (Utilities|GetClass OtherActor) "/Game/Blueprints/BP_Forninho.BP_Forninho_C")
    (CallFunction|SetRunningState false)
    (Rendering|Components|Sprite|SetSprite (Variables|Default|GetStandardSprite) "/Game/Sprites/SP_Forninho_Segurando3.SP_Forninho_Segurando3")))

(event EventTick
  (params (DeltaSeconds :type Float%20%28single-precision%29))
  (bind _xdestination (Variables|Default|GetXDestination))
  (bind _defaultsceneroot (Variables|Default|GetDefaultSceneRoot))
  (bind _returnvalue (Transformation|GetWorldLocation _defaultsceneroot))
  (bind _returnvalue_2 (- _xdestination (.x _returnvalue)))
  (bind _returnvalue_3 (< _returnvalue_2 0.0))
  (CallFunction|Animation)
  (if (Variables|Default|GetWalking)
    (if (< (Math|Float|Absolute(Float) _returnvalue_2) 2.0)
      (Variables|Default|SetCurrentSpeed 0.0)
      (bind _output_get (Variables|Default|SetWalking false))
      (CallFunction|SetRunningState _output_get)
      (else
        (Variables|Default|SetCurrentSpeed (* (Math|Integer|SelectInt -1 1 _returnvalue_3) (Variables|Default|GetSpeed)))
        (Transformation|SetActorRotation (Math|Rotator|MakeRotator 0.0 0.0 (Math|Float|SelectFloat 1.8e+02 0.0 _returnvalue_3)))
        (Transformation|AddActorWorldOffset (Math|Vector|MakeVector (* (Variables|Default|GetCurrentSpeed) (Utilities|Time|GetWorldDeltaSeconds)) 0.0 0.0))))))

(event EventBeginPlay
  (bind _asgm_forninho (Utilities|Casting|CastToGM_Forninho (Game|GetGameMode)))
  (bind _output_get (Variables|Default|SetMaxAnimationTimer (/ (Variables|/Game/Base/GM_MicroGame.GM_MicroGame_C|GetMax%20Time _asgm_forninho) 2e+01)))
  (Variables|Default|SetAnimationTimer _output_get)
  (Variables|Default|SetArmRot (Math|Rotator|MakeRotator 0.0 (/ 9e+01 _output_get) 0.0))
  (Variables|Default|SetLegRot (Math|Rotator|MakeRotator 0.0 (/ 6e+01 _output_get) 0.0)))

(event Input|TouchEvents|InputTouch
  (params (Location :type Vector) (FingerIndex :type ETouchIndex%20Enum))
  (bind (_x _y) (Math|Vector|BreakVector Location))
  (:Pressed
    (Variables|Default|SetXDestination (.X (Math|Vector|BreakVector (.WorldLocation (Class|PlayerController|DeprojectScreenPositiontoWorld (Game|GetPlayerController 0) _x _y)))) :!label _label)
    (if (not (Variables|Default|GetWalking))
      (bind _output_get (Variables|Default|SetWalking true))
      (CallFunction|SetRunningState _output_get)))
  (:Moved
    (goto _label)))

(fn ConstructionScript)

(fn ToggleSpriteType
  (Rendering|ToggleVisibility (Variables|Default|GetHead) false)
  (Rendering|ToggleVisibility (Variables|Default|GetLArm3) false)
  (Rendering|ToggleVisibility (Variables|Default|GetLArm1) false)
  (Rendering|ToggleVisibility (Variables|Default|GetLArm2) false)
  (Rendering|ToggleVisibility (Variables|Default|GetRArm3) false)
  (Rendering|ToggleVisibility (Variables|Default|GetRArm1) false)
  (Rendering|ToggleVisibility (Variables|Default|GetRArm2) false)
  (Rendering|ToggleVisibility (Variables|Default|GetLPerna1) false)
  (Rendering|ToggleVisibility (Variables|Default|GetLPerna2) false)
  (Rendering|ToggleVisibility (Variables|Default|GetRLeg1) false)
  (Rendering|ToggleVisibility (Variables|Default|GetRPerna2) false)
  (Rendering|ToggleVisibility (Variables|Default|GetWalkingSprite) false)
  (Rendering|ToggleVisibility (Variables|Default|GetStandardSprite) false))

(fn SetRunningState
  (params (IsRunning :type Boolean))
  (Rendering|SetVisibility (Variables|Default|GetStandardSprite) (not IsRunning) true)
  (Rendering|SetVisibility (Variables|Default|GetWalkingSprite) IsRunning true))

(fn Animation
  (bind _output_get (Variables|Default|SetAnimationTimer (- (Variables|Default|GetAnimationTimer) (Utilities|Time|GetWorldDeltaSeconds))))
  (if (<= _output_get 0.0)
    (Variables|Default|SetAnimationTimer (Variables|Default|GetMaxAnimationTimer))
    (Variables|Default|SetArmRot (* (Variables|Default|GetArmRot) -1))
    (Variables|Default|SetLegRot (* (Variables|Default|GetLegRot) -1))
    (else
      (Transformation|AddRelativeRotation (Variables|Default|GetLArm2) (* (Variables|Default|GetArmRot) (Utilities|Time|GetWorldDeltaSeconds)) false false)
      (Transformation|AddRelativeRotation (Variables|Default|GetLArm1) (* (* (Variables|Default|GetArmRot) (Utilities|Time|GetWorldDeltaSeconds)) 0.5) false false)
      (Transformation|AddRelativeRotation (Variables|Default|GetRArm2) (* (* (Variables|Default|GetArmRot) (Utilities|Time|GetWorldDeltaSeconds)) -1.0) false false)
      (Transformation|AddRelativeRotation (Variables|Default|GetRArm1) (* (* (Variables|Default|GetArmRot) (Utilities|Time|GetWorldDeltaSeconds)) -0.5) false false)
      (Transformation|AddRelativeRotation (Variables|Default|GetLPerna2) (* (* (Variables|Default|GetLegRot) (Utilities|Time|GetWorldDeltaSeconds)) 1.0) false false)
      (Transformation|AddRelativeRotation (Variables|Default|GetLPerna1) (* (* (Variables|Default|GetLegRot) (Utilities|Time|GetWorldDeltaSeconds)) 0.5) false false)
      (Transformation|AddRelativeRotation (Variables|Default|GetRPerna2) (* (* (Variables|Default|GetArmRot) (Utilities|Time|GetWorldDeltaSeconds)) -1.0) false false)
      (Transformation|AddRelativeRotation (Variables|Default|GetRLeg1) (* (* (Variables|Default|GetArmRot) (Utilities|Time|GetWorldDeltaSeconds)) -0.5) false false))))