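; BP_Shia is an animated Shia actor that plays a short timed sequence paced by the game instance's MicroGameTime.
; Tick counts down a timer and switches on AnimationPhase, first rotating BD and BE in opposite directions.
; When time runs out it swaps the Cbc sprite, activates SDoIt and waits half the original time.
; It then swaps visibility from Corpo to Corpo2 and disables its tick.
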(event EventBeginPlay
  (bind _asbp_guido_instance (Utilities|Casting|CastToBP_GuidoInstance (Game|GetGameInstance)))
  (bind _output_get (Variables|Default|SetMaxTime (/ (Variables|/Game/Base/BP_GuidoInstance.BP_GuidoInstance_C|GetMicroGame%20Time _asbp_guido_instance) 1.0)))
  (Variables|Default|SetTimer _output_get))

(event EventActorBeginOverlap
  (params (OtherActor :type Actor%20Object%20Reference)))

(event EventTick
  (params (DeltaSeconds :type Float%20%28single-precision%29))
  (Variables|Default|SetTimer (- (Variables|Default|GetTimer) DeltaSeconds))
  (switch int (Variables|Default|GetAnimationPhase)
    (:0
      (CallFunction|AddRotationOffset (Variables|Default|GetBD) (Variables|Default|GetAnimRot1) false)
      (CallFunction|AddRotationOffset (Variables|Default|GetBE) (Variables|Default|GetAnimRot1) true)
      (if (<= (Variables|Default|GetTimer) 0.0)
        (Math|Integer|IncrementInt (Variables|Default|GetAnimationPhase)
          (:%20%20
            (Rendering|Components|Sprite|SetSprite (Variables|Default|GetCbc) "/Game/Sprites/SP_Shia_Cbc2.SP_Shia_Cbc2")
            (Variables|Default|SetTimer (/ (Variables|Default|GetMaxTime) 2.0))
            (Components|Activation|Activate (Variables|Default|GetS_Do_it) false)))))
    (:1
      (if (<= (Variables|Default|GetTimer) 0.0)
        (Math|Integer|IncrementInt (Variables|Default|GetAnimationPhase)
          (:%20%20
            (Rendering|SetVisibility (Variables|Default|GetCorpo) false true)
            (Rendering|SetVisibility (Variables|Default|GetCorpo2) true true)
            (Actor|Tick|SetActorTickEnabled false)))))))

(fn ConstructionScript)

(fn AddRotationOffset
  (params (Component :type Scene%20Component%20Object%20Reference) (Rotator :type Rotator) (Sub :type Boolean))
  (Transformation|AddRelativeRotation Component (* Rotator (* (Math|Integer|SelectInt -1 1 Sub) (Utilities|Time|GetWorldDeltaSeconds))) false false))