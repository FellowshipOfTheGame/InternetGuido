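; BP_BarraMantem2D is a bar with a sliding marker that registers itself with the player pawn BP_GiovannaSegura on BeginPlay.
; SetPosition maps a progress value linearly onto the Slider's vertical offset, centered on the middle of the bar.
; IsGreen reports whether the Slider sits within the central band, the middle third of the travel for a 0–1 progress.
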(event EventBeginPlay
  (bind _asbp_giovanna_segura (Utilities|Casting|CastToBP_GiovannaSegura (Game|Player|GetPlayerPawn 0)))
  (Variables|/Game/Blueprints/BP_GiovannaSegura.BP_GiovannaSegura_C|SetBarra _asbp_giovanna_segura self))

(event Collision|EventActorBeginOverlap
  (params (OtherActor :type Actor%20Object%20Reference)))

(event EventTick
  (params (DeltaSeconds :type Float%20%28single-precision%29)))

(fn ConstructionScript)

(fn IsGreen
  (return (<= (Math|Float|Absolute(Float) (.Z (Math|Vector|BreakVector (Variables|/Script/Engine.SceneComponent|GetRelativeLocation (Variables|Default|GetSlider))))) 8e+01)))

(fn SetPosition
  (params (Progress :type Float%20%28single-precision%29))
  (Transformation|SetRelativeLocation (Variables|Default|GetSlider) (Math|Vector|MakeVector 0.0 1e+01 (- (* Progress 4.8e+02) 2.4e+02)) false false))