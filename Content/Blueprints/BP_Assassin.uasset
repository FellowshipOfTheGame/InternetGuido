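; Player-controlled assassin who strikes a victim with a spoon on timed taps, winning through GM_Murder once the difficulty-based hit count runs out.
; A touch inside the ActionBar's green zone starts a staged, Tick-driven arm swing, alongside a looping walk bob.
; Each hit notifies the victim and either bends the spoon and reveals a tweened render-target camera view, or destroys the spoon on the last.
; Animation speeds derive from the game mode's MaxTime.
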(event EventTick
  (params (DeltaSeconds :type Float%20%28single-precision%29))
  (Variables|Default|SetAnimation%20Counter (- (Variables|Default|GetAnimation%20Counter) DeltaSeconds))
  (Variables|Default|SetWalking%20Timer (- (Variables|Default|GetWalking%20Timer) DeltaSeconds))
  (CallFunction|RelativeRotationOffset (Variables|Default|GetLArm) (* (Variables|Default|GetLArmRotation) (Utilities|Time|GetWorldDeltaSeconds)))
  ;[1 1 1] Walking Animation
  (Transformation|AddActorWorldOffset (* (Variables|Default|GetTransladation%20Velocity) (Utilities|Time|GetWorldDeltaSeconds)))
  (if (<= (Variables|Default|GetWalking%20Timer) 0.0)
    (Variables|Default|SetTransladation%20Velocity (* (Variables|Default|GetTransladation%20Velocity) -1))
    (Variables|Default|SetLArmRotation (* (Variables|Default|GetLArmRotation) -1.0))
    (Variables|Default|SetWalking%20Timer (Variables|Default|GetDefault%20Walking)))
  ;[1 1 1] Rising Arm Animation
  (CallFunction|RelativeRotationOffset (Variables|Default|GetForearm) (* (Variables|Default|GetForearmRotation) (Utilities|Time|GetWorldDeltaSeconds)))
  (CallFunction|RelativeRotationOffset (Variables|Default|GetArm) (* (Variables|Default|GetArmRotation) (Utilities|Time|GetWorldDeltaSeconds)))
  (switch int (Variables|Default|GetAnimation%20Stage)
    (:1
      (if (<= (Variables|Default|GetAnimation%20Counter) 0.0)
        (Variables|Default|SetArmRotation (Math|Rotator|MakeRotator 0.0 (/ -2e+02 (/ (Variables|Default|GetDefault%20Arm) 2.0)) 0.0))
        (Variables|Default|SetForearmRotation (Math|Rotator|MakeRotator 0.0 (/ -6e+01 (/ (Variables|Default|GetDefault%20Arm) 4.0)) 0.0))
        (Variables|Default|SetAnimation%20Stage 2)
        (Variables|Default|SetAnimation%20Counter (/ (Variables|Default|GetDefault%20Arm) 4.0))))
    (:2
      (if (<= (Variables|Default|GetAnimation%20Counter) 0.0)
        (Variables|Default|SetForearmRotation (* (Variables|Default|GetForearmRotation) -1.0))
        (Variables|Default|SetAnimation%20Stage 3)
        (Variables|Default|SetAnimation%20Counter (/ (Variables|Default|GetDefault%20Arm) 4.0))
        (Default|SpoonHit (Variables|Default|GetVictin))
        (bind _result (Math|Integer|DecrementInt (Variables|Default|GetHits))
          (:%20%20
            (if (> _result 0)
              (CallFunction|CreateCamera)
              (CallFunction|RelativeRotationOffset (Variables|Default|GetSpoon) (Variables|Default|GetSpoonRotation))
              (else
                (bind _asgm_murder (Utilities|Casting|CastToGM_Murder (Game|GetGameMode)))
                (Default|Win _asgm_murder)
                (Components|DestroyComponent (Variables|Default|GetSpoon))))))))
    (:3
      (if (<= (Variables|Default|GetAnimation%20Counter) 0.0)
        (Variables|Default|SetArmRotation "0, 0, 0")
        (Variables|Default|SetForearmRotation "0, 0, 0")
        (Variables|Default|SetAnimation%20Stage 0)))))

(event EventBeginPlay
  ;[1 1 1] Begin Play
  (bind _asgm_murder (Utilities|Casting|CastToGM_Murder (Game|GetGameMode)))
  (Variables|Default|SetDefault%20Arm (* (Variables|/Game/Base/GM_MicroGame.GM_MicroGame_C|GetMax%20Time _asgm_murder) 0.1))
  (bind _output_get (Variables|Default|SetDefault%20Walking (* (Variables|/Game/Base/GM_MicroGame.GM_MicroGame_C|GetMax%20Time _asgm_murder) 0.1)))
  (Variables|Default|SetTransladation%20Velocity (Math|Vector|MakeVector 0.0 0.0 (/ 1e+02 _output_get)))
  (Variables|Default|SetWalking%20Timer (Variables|Default|GetDefault%20Walking))
  (Variables|Default|SetLArmRotation (Math|Rotator|MakeRotator 0.0 (/ 2e+01 (Variables|Default|GetDefault%20Walking)) 0.0))
  (bind _asbp_guido_instance (Utilities|Casting|CastToBP_GuidoInstance (Game|GetGameInstance)))
  (bind _output_get_2 (Variables|Default|SetMaxHits (+ (Variables|/Game/Base/BP_GuidoInstance.BP_GuidoInstance_C|GetDificulty _asbp_guido_instance) 1)))
  (Variables|Default|SetHits _output_get_2)
  (Variables|Default|SetSpoonRotation (Math|Rotator|MakeRotator 0.0 (/ 9e+01 (Math|Conversions|ToFloat(Integer) _output_get_2)) 0.0)))

(event Input|TouchEvents|InputTouch
  (params (Location :type Vector) (FingerIndex :type ETouchIndex%20Enum))
  (:Pressed
    (if (Default|IsinGreenZone (Variables|Default|GetActionBar))
      (if (and (== (Variables|Default|GetAnimation%20Stage) 0) (> (Variables|Default|GetHits) 0))
        (Variables|Default|SetArmRotation (Math|Rotator|MakeRotator 0.0 (/ 2e+02 (Variables|Default|GetDefault%20Arm)) 0.0))
        (Variables|Default|SetAnimation%20Stage 1)
        (Variables|Default|SetAnimation%20Counter (Variables|Default|GetDefault%20Arm))
        (Development|PrintString "Touch")))))

(fn ConstructionScript)

(fn RelativeRotationOffset
  (params (Component :type Scene%20Component%20Object%20Reference) (Ofsset :type Rotator))
  (Transformation|SetRelativeRotation Component (Math|Rotator|CombineRotators Ofsset (Variables|/Script/Engine.SceneComponent|GetRelativeRotation Component)) false false))

(fn CreateCamera
  (bind _hits (Variables|Default|GetHits))
  (bind _maxhits (Variables|Default|GetMaxHits))
  (bind _cameras (Variables|Default|GetCameras))
  (bind _returnvalue (- _maxhits _hits))
  (bind _returnvalue_2 (- _returnvalue 1))
  (bind _item (Utilities|Array|Get(acopy) _cameras _returnvalue_2))
  (bind _returnvalue_3 (Utilities|Select :Index _returnvalue_2 :Option%200 "/Game/Base/Materials/CameraRender1.CameraRender1" :Option%201 "/Game/Base/Materials/CameraRender2.CameraRender2" :Option%202 "/Game/Base/Materials/CameraRender3.CameraRender3"))
  (Development|PrintString (Utilities|String|ToString(Integer) _returnvalue_2))
  (Rendering|SetVisibility (Variables|/Game/Blueprints/BP_CloseUp.BP_CloseUp_C|GetCube _item) true false)
  (Rendering|SetVisibility (Variables|/Game/Blueprints/BP_CloseUp.BP_CloseUp_C|GetFrame _item) true false)
  (Variables|/Script/Engine.SceneCaptureComponent2D|SetTextureTarget (Variables|/Game/Blueprints/BP_CloseUp.BP_CloseUp_C|GetSceneCaptureComponent2D _item) _returnvalue_3)
  (Rendering|Material|SetTextureParameterValue (Variables|/Game/Blueprints/BP_CloseUp.BP_CloseUp_C|GetMaterial _item) "Renderer" _returnvalue_3)
  (Variables|/Game/Blueprints/BP_CloseUp.BP_CloseUp_C|SetCameraTarget _item (Utilities|Select :Index _returnvalue_2 :Option%200 (Variables|Default|GetSpoonTarget) :Option%201 (Variables|/Game/Blueprints/BP_Victin.BP_Victin_C|GetVictin%20Target (Variables|Default|GetVictin)) :Option%202 (Variables|Default|GetHeadTarget)))
  (Default|Tween _item))