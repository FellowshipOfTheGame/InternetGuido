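; Background sprite actor that the player's cat can swap or fade out.
; On BeginPlay it registers itself as the Background reference on the player BP_Cat pawn.
; ChangeSprite replaces the displayed sprite, and the Vanish event runs a two-second color tween on it through BPTweenComponent using the GoneAlpha curve.
; Nothing inside this Blueprint triggers either one.
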(event Custom|Vanish
  (Default|SpriteColorTween (Variables|Default|GetBP_TweenComponent) "/Game/Curves/GoneAlpha.GoneAlpha" (Variables|Default|GetBackground) 2.0 "1,1,1" 1.0 0.0 3e+01))

(event EventBeginPlay
  (bind _asbp_cat (Utilities|Casting|CastToBP_Cat (Game|Player|GetPlayerPawn 0)))
  (Variables|/Game/Blueprints/BP_Cat.BP_Cat_C|SetBackground _asbp_cat self))

(event Collision|EventActorBeginOverlap
  (params (OtherActor :type Actor%20Object%20Reference)))

(fn ConstructionScript)

(fn ChangeSprite
  (params (Sprite :type Paper%20Sprite%20Object%20Reference))
  (Rendering|Components|Sprite|SetSprite (Variables|Default|GetBackground) Sprite))