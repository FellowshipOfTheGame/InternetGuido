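; BP_Ape is a sprite ape that the player flips left or right by touch, with shoot and victory reactions.
; BeginPlay derives a flip cooldown from GM_Ape's MaxTime, and Tick runs that cooldown to re-enable input.
; Tick also checks a random shoot timer, re-randomized every frame as wired; Shoot only plays a recoil scale tween.
; BPTweenComponent drives the bouncing flip and recoil; Win stops Tick and swaps in the victory sprite.
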(event Custom|Win
  ;[1 1 1] Win Pose
  (Development|PrintString "Você ganhou")
  (Actor|Tick|SetActorTickEnabled false)
  (Rendering|Components|Sprite|SetSprite (Variables|Default|GetSprite) "/Game/Sprites/SP_Ape_Victory.SP_Ape_Victory"))

(event Custom|Shoot
  ;[1 1 1] Shooting
  (Default|ScaleTween (Variables|Default|GetBP_TweenComponent) "/Game/Curves/Shooting.Shooting" (Variables|Default|GetSprite) 1.0 "1, 1, 1" "1, 1, 1" 0.0 3e+01) ; Shoot Recoil
)

(event EventBeginPlay
  ;[1 1 1] Set random time for Shooting
  (Variables|Default|SetRandomShootTime (Math|Random|RandomFloatinRange 0.5 1.0))
  (bind _asgm_ape (Utilities|Casting|CastToGM_Ape (Game|GetGameMode)))
  (Variables|Default|SetMaxDelayTime (/ 1e+01 (Variables|/Game/Base/GM_MicroGame.GM_MicroGame_C|GetMax%20Time _asgm_ape)))
  (Variables|Default|SetDelayCounter 0.0)
  (Variables|Default|SetCanShoot true))

(event EventTick
  (params (DeltaSeconds :type Float%20%28single-precision%29))
  ;[1 1 1] Update Shooting Time
  (bind _output_get (Variables|Default|SetRandomShootTime (- (stale _output_get) DeltaSeconds)))
  (if (<= _output_get 0.0)
    (CallFunction|Shoot))
  (Variables|Default|SetRandomShootTime (Math|Random|RandomFloatinRange 3.0 8.0))
  (if (>= (+ (Variables|Default|GetDelayCounter) (Utilities|Time|GetWorldDeltaSeconds)) (Variables|Default|GetMaxDelayTime))
    (Variables|Default|SetCanShoot true))
  (Variables|Default|SetDelayCounter (Math|Float|SelectFloat 0.0 (+ (Variables|Default|GetDelayCounter) (Utilities|Time|GetWorldDeltaSeconds)) (>= (+ (Variables|Default|GetDelayCounter) (Utilities|Time|GetWorldDeltaSeconds)) (Variables|Default|GetMaxDelayTime)))))

(event Input|TouchEvents|InputTouch
  (params (Location :type Vector) (FingerIndex :type ETouchIndex%20Enum))
  ;[1 1 1] Rotation
  (:Pressed
    (if (Variables|Default|GetCanShoot)
      (Default|RotationTween (Variables|Default|GetBP_TweenComponent) "/Game/Curves/OutBounce.OutBounce" (Variables|Default|GetRoot) (Math|Rotator|MakeRotator 0.0 0.0 (select (Variables|Default|GetIsRight) 0.0 1.8e+02)) (Math|Rotator|MakeRotator 0.0 0.0 (select (Variables|Default|GetIsRight) 1.8e+02 0.0)) "NewEnumerator1" 1.0 "1.000000, 1, 1" 0.0 3e+01 false)
      (Variables|Default|SetIsRight (not (Variables|Default|GetIsRight)))
      (Variables|Default|SetCanShoot false))))

(fn ConstructionScript)