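; BP_BackGround is an endlessly scrolling sprite background with selectable artwork.
; On BeginPlay it shows both scrolling sprites, derives their speed from GM_Murder's MaxTime, and applies the sprite chosen by Version to them and a Preview sprite.
; Each Tick moves the left and right sprites along negative X, wrapping either back to the opposite edge once it passes the limit, forming a two-tile loop.
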(event EventBeginPlay
  (Rendering|SetVisibility (Variables|Default|GetLeftSprite) true false)
  (Rendering|SetVisibility (Variables|Default|GetRightSprite) true false)
  (bind _asgm_murder (Utilities|Casting|CastToGM_Murder (Game|GetGameMode))
    (:then
      (Variables|Default|SetScrollig%20Speed (* (/ (Variables|/Game/Base/GM_MicroGame.GM_MicroGame_C|GetMax%20Time _asgm_murder) 1e+01) 1e+02)))
    (:CastFailed
      _))
  (CallFunction|SelectVersion (Variables|Default|GetVersion)))

(event EventTick
  (params (DeltaSeconds :type Float%20%28single-precision%29))
  (bind _scrollig_speed (Variables|Default|GetScrollig%20Speed))
  (bind _leftsprite (Variables|Default|GetLeftSprite))
  (bind _rightsprite (Variables|Default|GetRightSprite))
  (bind _leftsprite_2 (Variables|Default|GetLeftSprite))
  (bind _rightsprite_2 (Variables|Default|GetRightSprite))
  (bind _returnvalue (* DeltaSeconds _scrollig_speed))
  (bind _returnvalue_2 (* "-1.000000,0.000000,0.000000" _returnvalue))
  (Transformation|SetRelativeLocation _leftsprite (+ _returnvalue_2 (Variables|/Script/Engine.SceneComponent|GetRelativeLocation _leftsprite)) false false)
  (Transformation|SetRelativeLocation _rightsprite_2 (+ _returnvalue_2 (Variables|/Script/Engine.SceneComponent|GetRelativeLocation _rightsprite_2)) false false)
  (if (<= (.x (Variables|/Script/Engine.SceneComponent|GetRelativeLocation _leftsprite_2)) -1024.0)
    (Transformation|SetRelativeLocation _leftsprite_2 "1024.000000,0.000000,0.000000" false false))
  (if (<= (.x (Variables|/Script/Engine.SceneComponent|GetRelativeLocation _rightsprite)) -1024.0)
    (Transformation|SetRelativeLocation _rightsprite "1024.000000, 0,0.000000" false false)))

(fn ConstructionScript)

(fn SelectVersion
  (params (Version :type Integer))
  (bind _returnvalue (Utilities|Select :Index Version :Option%200 "/Game/Sprites/SP_Egypt.SP_Egypt" :Option%201 "/Game/Sprites/SP_grin_riu_zoune.SP_grin_riu_zoune"))
  (Rendering|Components|Sprite|SetSprite (Variables|Default|GetLeftSprite) _returnvalue)
  (Rendering|Components|Sprite|SetSprite (Variables|Default|GetRightSprite) _returnvalue)
  (Rendering|Components|Sprite|SetSprite (Variables|Default|GetPreview) _returnvalue))