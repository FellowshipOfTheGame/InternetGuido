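; World-space progress bar actor built from a red bar and a green bar that shows the filled amount.
; The construction script tints each bar through its own dynamic instance of M_Cable.
; SetScale hides the green bar at zero or below, otherwise caps the value at one, scales X and shifts X by minus half so it grows from one end.
; BeginPlay starts the bar empty.
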(event EventBeginPlay
  (CallFunction|SetScale 0.0))

(event EventActorBeginOverlap
  (params (OtherActor :type Actor%20Object%20Reference)))

(event EventTick
  (params (DeltaSeconds :type Float%20%28single-precision%29)))

(fn ConstructionScript
  (bind _returnvalue (Rendering|Material|CreateDynamicMaterialInstance "/Game/Materials/M_Cable.M_Cable" :!class /Script/Engine.KismetMaterialLibrary))
  (Rendering|Material|SetVectorParameterValue _returnvalue "Color" (Utilities|Struct|MakeLinearColor 1.0 0.0 0.0 1.0) :!class /Script/Engine.MaterialInstanceDynamic)
  (Rendering|Material|SetMaterial (Variables|Default|GetRedBar) 0 _returnvalue)
  (bind _returnvalue_2 (Rendering|Material|CreateDynamicMaterialInstance "/Game/Materials/M_Cable.M_Cable" :!class /Script/Engine.KismetMaterialLibrary))
  (Rendering|Material|SetVectorParameterValue _returnvalue_2 "Color" (Utilities|Struct|MakeLinearColor 0.0 1.0 0.0 1.0) :!class /Script/Engine.MaterialInstanceDynamic)
  (Rendering|Material|SetMaterial (Variables|Default|GetGreenBar) 0 _returnvalue_2))

(fn SetScale
  (params (Scale :type Float%20%28single-precision%29))
  (bind _returnvalue (<= Scale 1.0))
  (bind _returnvalue_2 (> Scale 0.0))
  (bind _greenbar (Variables|Default|GetGreenBar))
  (bind _returnvalue_3 (Math|Float|SelectFloat Scale 1.0 _returnvalue))
  (bind _relativescale3d (Variables|/Script/Engine.SceneComponent|GetRelativeScale3D _greenbar))
  (bind _relativelocation (Variables|/Script/Engine.SceneComponent|GetRelativeLocation _greenbar))
  (Rendering|SetVisibility (Variables|Default|GetGreenBar) _returnvalue_2 false)
  (if _returnvalue_2
    (Transformation|SetRelativeScale3D _greenbar (Math|Vector|MakeVector _returnvalue_3 (.y _relativescale3d) (.z _relativescale3d)))
    (Transformation|SetRelativeLocation _greenbar (Math|Vector|MakeVector (/ _returnvalue_3 -2.0) (.y _relativelocation) (.z _relativelocation)) false false)))