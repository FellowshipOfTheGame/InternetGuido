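; BP_ActionBar is a timing-bar actor with a marker sweeping over red and green zones, registered with the player's BP_Assassin on BeginPlay.
; The green zone narrows as the game instance's difficulty rises, and Tick bounces the yellow Scroll marker between the bar's ends.
; IsInGreenZone reports whether the marker is within the green zone; the touch handler repeats this test but does nothing with it.
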(event EventBeginPlay
  (bind _asbp_guido_instance (Utilities|Casting|CastToBP_GuidoInstance (Game|GetGameInstance)))
  (Transformation|SetRelativeScale3D (Variables|Default|GetGreenBar) (Math|Vector|MakeVector (* (- 4 (Variables|/Game/Base/BP_GuidoInstance.BP_GuidoInstance_C|GetDificulty _asbp_guido_instance)) 0.25) 2.0 1.0))
  (bind _asbp_assassin (Utilities|Casting|CastToBP_Assassin (Game|Player|GetPlayerPawn 0)))
  (Variables|/Game/Blueprints/BP_Assassin.BP_Assassin_C|SetActionBar _asbp_assassin self))

(event EventActorBeginOverlap
  (params (OtherActor :type Actor%20Object%20Reference)))

(event EventTick
  (params (DeltaSeconds :type Float%20%28single-precision%29))
  (Transformation|AddLocalOffset (Variables|Default|GetScroll) (Math|Vector|MakeVector (* DeltaSeconds (Variables|Default|GetSpeed)) 0.0 0.0) false false)
  (if (>= (Math|Float|Absolute(Float) (.X (Math|Vector|BreakVector (Variables|/Script/Engine.SceneComponent|GetRelativeLocation (Variables|Default|GetScroll))))) 5e+01)
    (Variables|Default|SetSpeed (* -1 (Variables|Default|GetSpeed)))))

(event Input|TouchEvents|InputTouch
  (params (Location :type Vector) (FingerIndex :type ETouchIndex%20Enum))
  (:Pressed
    (if (<= (Math|Float|Absolute(Float) (.X (Math|Vector|BreakVector (Variables|/Script/Engine.SceneComponent|GetRelativeLocation (Variables|Default|GetScroll))))) (* 50 (.X (Math|Vector|BreakVector (Variables|/Script/Engine.SceneComponent|GetRelativeScale3D (Variables|Default|GetGreenBar))))))
      _)))

(fn ConstructionScript
  (bind _returnvalue (Rendering|Material|CreateDynamicMaterialInstance "/Game/Base/Materials/M_Cable.M_Cable" :!class /Script/Engine.KismetMaterialLibrary))
  (Rendering|Material|SetVectorParameterValue _returnvalue "Color" (Utilities|Struct|MakeLinearColor 1.0 0.0 0.0 1.0) :!class /Script/Engine.MaterialInstanceDynamic)
  (Rendering|Material|SetMaterial (Variables|Default|GetRedBar) 0 _returnvalue)
  (bind _returnvalue_2 (Rendering|Material|CreateDynamicMaterialInstance "/Game/Base/Materials/M_Cable.M_Cable" :!class /Script/Engine.KismetMaterialLibrary))
  (Rendering|Material|SetVectorParameterValue _returnvalue_2 "Color" (Utilities|Struct|MakeLinearColor 0.0 1.0 0.0 1.0) :!class /Script/Engine.MaterialInstanceDynamic)
  (Rendering|Material|SetMaterial (Variables|Default|GetGreenBar) 0 _returnvalue_2)
  (bind _returnvalue_3 (Rendering|Material|CreateDynamicMaterialInstance "/Game/Base/Materials/M_Cable.M_Cable" :!class /Script/Engine.KismetMaterialLibrary))
  (Rendering|Material|SetVectorParameterValue _returnvalue_3 "Color" (Utilities|Struct|MakeLinearColor 1.0 1.0 0.0 1.0) :!class /Script/Engine.MaterialInstanceDynamic)
  (Rendering|Material|SetMaterial (Variables|Default|GetScroll) 0 _returnvalue_3))

(fn IsinGreenZone
  (return (<= (Math|Float|Absolute(Float) (.X (Math|Vector|BreakVector (Variables|/Script/Engine.SceneComponent|GetRelativeLocation (Variables|Default|GetScroll))))) (* 50 (.X (Math|Vector|BreakVector (Variables|/Script/Engine.SceneComponent|GetRelativeScale3D (Variables|Default|GetGreenBar))))))))