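; BP_Torrada is a toast actor that can bounce and be eaten by moving into a mouth position.
; Bounce runs a scale tween on the Torrada component through BPTweenComponent.
; Shrink starts a translation tween from the actor's location to the given mouth position alongside a scale-down tween, then calls Die, which destroys the actor after a one-second delay.
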(event Custom|Bounce
  (Default|ScaleTween (Variables|Default|GetBP_TweenComponent) "/Game/Curves/Select.Select" (Variables|Default|GetTorrada) 1.0 "1, 1, 1" "1, 1, 1" 0.0 3e+01))

(event Custom|Die
  (Utilities|FlowControl|Delay 1.0)
  (Actor|DestroyActor))

(event EventBeginPlay)

(event EventTick
  (params (DeltaSeconds :type Float%20%28single-precision%29)))

(fn ConstructionScript)

(fn Shrink
  (params (Mouth :type Vector))
  (bind _self self)
  (bind _output_get (LocalVariables|SetInitialPos (Transformation|GetActorLocation)))
  (Default|TranslationTween (Variables|Default|GetBP_TweenComponent) "/Game/Curves/Linear.Linear" _self _output_get Mouth "NewEnumerator1" 1.0 "0.500000,0.500000,0.500000" 0.0 3e+01)
  (Default|ScaleTween (Variables|Default|GetBP_TweenComponent) "/Game/Curves/DownCurve.DownCurve" _self 1.0 "1, 1, 1" "1, 1, 1" 0.0 3e+01)
  (CallFunction|Die))