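; BP_Bee is a touchable bee actor that makes the player lose when tapped in the cage game.
; A touch calls FoiClicado only if the Clicado flag is set and the GM_Cage game mode has not registered a win.
; FoiClicado toggles NCage's visibility, clears the flag to block repeat triggers, calls Lose on the game mode and activates the NotTheBees component.
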(event Custom|FoiClicado
  (Rendering|ToggleVisibility (Variables|Default|GetNCage) false)
  (Variables|Default|SetClicado false)
  (bind _asgm_cage (Utilities|Casting|CastToGM_Cage (Game|GetGameMode)))
  (Default|Lose _asgm_cage)
  (Components|Activation|Activate (Variables|Default|GetNotTheBees) false))

(event EventActorOnInputTouchBegin
  (params (FingerIndex :type ETouchIndex%20Enum :default "Touch1"))
  (bind _asgm_cage (Utilities|Casting|CastToGM_Cage (Game|GetGameMode)))
  (if (and (Variables|Default|GetClicado) (not (Variables|/Game/Gamemodes/GM_Cage.GM_Cage_C|GetWon _asgm_cage)))
    (CallFunction|FoiClicado)))

(fn ConstructionScript)