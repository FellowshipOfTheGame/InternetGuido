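; Clock timing minigame for GM_Hammer: the minute hand spins until a tap stops it, winning if it lands near a marked hour.
; BeginPlay randomizes the hour hand, picks consecutive target hours whose count depends on GameInstance difficulty, and places sprites around the dial.
; Spin speed scales with the game mode's MaxTime.
; A tap compares the atan2-derived hand angle to each target with wraparound tolerance, reporting Win or Lost and changing music effects on a win.
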(event EventBeginPlay
  (Transformation|SetRelativeRotation (Variables|Default|GetPonteiroH) (Math|Rotator|MakeRotator 0.0 (* (Math|Random|RandomIntegerinRange 0 11) 3e+01) 0.0) false false)
  (bind _asgm_hammer (Utilities|Casting|CastToGM_Hammer (Game|GetGameMode))
    (:then
      _)
    (:CastFailed
      _))
  (Variables|Default|SetRadialVelocity (/ (* -3.6e+02 5.0) (Variables|/Game/Base/GM_MicroGame.GM_MicroGame_C|GetMax%20Time _asgm_hammer)))
  (Utilities|Array|Add (Variables|Default|GetClockHours) (Math|Random|RandomIntegerinRange 1 12))
  (Variables|Default|SetSong (Variables|/Game/Base/GM_MicroGame.GM_MicroGame_C|GetMusicPlayer _asgm_hammer))
  (bind _asbp_guido_instance (Utilities|Casting|CastToBP_GuidoInstance (Game|GetGameInstance)))
  (for _index (range 1 (- 3 (Variables|/Game/Base/BP_GuidoInstance.BP_GuidoInstance_C|GetDificulty _asbp_guido_instance)))
    (Utilities|Array|Add (Variables|Default|GetClockHours) (Math|Integer|SelectInt (- (+ (Utilities|Array|Get(acopy) (Variables|Default|GetClockHours)) _index) 12) (+ (Utilities|Array|Get(acopy) (Variables|Default|GetClockHours)) _index) (> (+ (Utilities|Array|Get(acopy) (Variables|Default|GetClockHours)) _index) 12))))
  (Variables|Default|SetRaio (.x (Variables|/Script/Engine.SceneComponent|GetRelativeLocation (Variables|Default|GetRadius))))
  (for _array_element (Variables|Default|GetClockHours)
    (AddComponent|AddPaperSpriteComponent false (Math|Transform|MakeTransform (Math|Vector|MakeVector (* (Math|Trig|Sin(Degrees) (* _array_element 3e+01)) (Variables|Default|GetRaio)) 0.0 (* (Variables|Default|GetRaio) (Math|Trig|Cos(Degrees) (* _array_element 3e+01)))) "0, 0, 0" "0.500000,1,0.500000"))
    (Effects|Components|ParticleSystem|SetIntParameter (Variables|Default|GetSong) "Effect" 0)))

(event EventActorBeginOverlap
  (params (OtherActor :type Actor%20Object%20Reference)))

(event EventTick
  (params (DeltaSeconds :type Float%20%28single-precision%29))
  (if (Variables|Default|GetRotating)
    (CallFunction|AddRotOffset (Variables|Default|GetPonteiroM) (Math|Rotator|MakeRotator 0.0 (* DeltaSeconds (Variables|Default|GetRadialVelocity)) 0.0))))

(event Input|TouchEvents|InputTouch
  (params (Location :type Vector) (FingerIndex :type ETouchIndex%20Enum))
  (bind _degrees (CallFunction|ClockDegree))
  (:Pressed
    (Variables|Default|SetRotating false)
    (Variables|Default|SetWon false)
    (bind _array_element (Utilities|Array|ForEachLoopwithBreak (Variables|Default|GetClockHours) :!label _label)
      (:LoopBody
        (Development|PrintString (Utilities|String|Append "Destino" (Utilities|String|ToString(Float) (* _array_element 3e+01)) "/Dado:" (Utilities|String|ToString(Float) _degrees)))
        (if (Utilities|ValueinRange _degrees (* _array_element 3e+01) 45.0)
          (Variables|Default|SetWon true)
          (goto _label Break)))
      (:Completed
        (bind _asgm_hammer (Utilities|Casting|CastToGM_Hammer (Game|GetGameMode)))
        (if (Variables|Default|GetWon)
          (Default|Win _asgm_hammer)
          (Effects|Components|ParticleSystem|SetIntParameter (Variables|Default|GetSong) "Effect" 1)
          (Utilities|FlowControl|Delay 1.3)
          (Effects|Components|ParticleSystem|SetIntParameter (Variables|Default|GetSong) "Effect" 2)
          (else
            (Default|Lost _asgm_hammer)))))))

(fn ConstructionScript)

(fn AddRotOffset
  (params (Component :type Scene%20Component%20Object%20Reference) (RotOfsset :type Rotator))
  (Transformation|SetRelativeRotation Component (Math|Rotator|CombineRotators (Variables|/Script/Engine.SceneComponent|GetRelativeRotation Component) RotOfsset) false false))

(fn ClockDegree
  (bind _returnvalue (Transformation|GetActorLocation))
  (bind _angle (Variables|Default|GetAngle))
  (bind _returnvalue_2 (Transformation|GetWorldLocation _angle))
  (bind _returnvalue_3 (- _returnvalue_2 _returnvalue))
  (bind _returnvalue_4 (Class|KismetMathLibrary|DegAtan2 (.x _returnvalue_3) (.z _returnvalue_3)))
  (return (Math|Float|SelectFloat (+ _returnvalue_4 3.6e+02) _returnvalue_4 (< _returnvalue_4 0.0))))