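; BP_CloseUp is a close-up camera actor whose SceneCapture2D follows a Target along world X and Z.
; On BeginPlay it hides its Cube and adds itself to the Cameras array on the player's BP_Assassin pawn.
; Each Tick, while Target is valid, it moves the capture component to the target's X and Z at a fixed world Y.
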(event EventBeginPlay
  (Rendering|SetVisibility (Variables|Default|GetCube) false false)
  (bind _asbp_assassin (Utilities|Casting|CastToBP_Assassin (Game|Player|GetPlayerPawn 0)))
  (Utilities|Array|Add (Variables|/Game/Blueprints/BP_Assassin.BP_Assassin_C|GetCameras _asbp_assassin) self))

(event EventActorBeginOverlap
  (params (OtherActor :type Actor%20Object%20Reference)))

(event EventTick
  (params (DeltaSeconds :type Float%20%28single-precision%29))
  (bind _target (Variables|Default|GetTarget))
  (bind _returnvalue (Transformation|GetWorldLocation _target))
  (if (Utilities|IsValid _target)
    (Transformation|SetWorldLocation (Variables|Default|GetSceneCaptureComponent2D) (Math|Vector|MakeVector (.x _returnvalue) 1.5e+02 (.z _returnvalue)) false false)))

(fn ConstructionScript)