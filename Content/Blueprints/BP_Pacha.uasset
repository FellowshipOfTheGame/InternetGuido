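; BP_Pacha is a touch-driven tuning minigame actor where the player slides a hand vertically to find the right tone.
; Touch input sets a target height from the deprojected screen position, and Tick moves the hand toward it at constant speed.
; RightTune checks nested tolerance bands to drive audio volume, noise and mouth sprites.
; Holding the innermost band for a fifth of GM_Pacha's MaxTime calls Win and stops ticking.
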(event Custom|Right%20Tune
  (bind _mouth (Variables|Default|GetMouth))
  ;[0.4757 0.695 1] Checks if the hand is in the right position
  (if (Utilities|IsinRange (* (Variables|Default|GetToleration) 3.0))
    (if (Utilities|IsinRange (* (Variables|Default|GetToleration) 2.0))
      (if (Utilities|IsinRange (Variables|Default|GetToleration))
        (if (Variables|Default|GetInTune)
          _
          (else
            (Variables|Default|SetInTune true)
            (Variables|Default|SetAssi%20counter 0.0)
            (Effects|Components|ParticleSystem|SetBoolParameter (Variables|Default|GetAudio) "Noise" false)
            (Rendering|Components|Sprite|SetSprite (Variables|Default|GetMouth) "/Game/Sprites/SP_PachaMounth_Right.SP_PachaMounth_Right")))
        (bind _output_get (Variables|Default|SetAssi%20counter (+ (Variables|Default|GetAssi%20counter) (Utilities|Time|GetWorldDeltaSeconds))))
        (if (>= _output_get (Variables|Default|GetAssimilation%20Time))
          (bind _asgm_pacha (Utilities|Casting|CastToGM_Pacha (Game|GetGameMode)))
          (Default|Win _asgm_pacha)
          (Actor|Tick|SetActorTickEnabled false))
        (else
          (Audio|Components|Audio|SetVolumeMultiplier (Variables|Default|GetAudio) 0.7 :!class /Script/Engine.AudioComponent)
          (Effects|Components|ParticleSystem|SetBoolParameter (Variables|Default|GetAudio) "Noise" true)
          (Variables|Default|SetInTune false)
          (Rendering|SetVisibility _mouth true false)
          (Rendering|Components|Sprite|SetSprite _mouth "/Game/Sprites/SP_PachaMouth_OK.SP_PachaMouth_OK")))
      (else
        (Audio|Components|Audio|SetVolumeMultiplier (Variables|Default|GetAudio) 0.3 :!class /Script/Engine.AudioComponent)
        (Effects|Components|ParticleSystem|SetIntParameter (Variables|Default|GetAudio) "Static" 1)
        (Rendering|SetVisibility (Variables|Default|GetMouth) false false)))
    (else
      (Audio|Components|Audio|SetVolumeMultiplier (Variables|Default|GetAudio) 0.1 :!class /Script/Engine.AudioComponent)
      (Effects|Components|ParticleSystem|SetBoolParameter (Variables|Default|GetAudio) "Noise" true)
      (Rendering|SetVisibility (Variables|Default|GetMouth) false false))))

(event EventTick
  (params (DeltaSeconds :type Float%20%28single-precision%29))
  (CallFunction|UpdateLocation (Variables|Default|GetHand) (Variables|Default|GetSpeed) (Variables|Default|GetTarget%20Location))
  (CallFunction|RightTune))

(event EventBeginPlay
  (Effects|Components|ParticleSystem|SetIntParameter (Variables|Default|GetAudio) "Chose" (Math|Random|RandomIntegerinRange 0 2))
  (bind _asgm_pacha (Utilities|Casting|CastToGM_Pacha (Game|GetGameMode)))
  (Variables|Default|SetAssimilation%20Time (* (Variables|/Game/Base/GM_MicroGame.GM_MicroGame_C|GetMax%20Time _asgm_pacha) 0.2)))

(event Input|TouchEvents|InputTouch
  (params (Location :type Vector) (FingerIndex :type ETouchIndex%20Enum))
  (bind _hand (Variables|Default|GetHand))
  (bind _returnvalue (Transformation|GetWorldLocation _hand))
  ;[1 1 1] Find Out desired Location
  (:Pressed
    (bind _asplayer_controller (Utilities|Casting|CastToPlayerController (Game|GetPlayerController 0) :!label _label))
    (Variables|Default|SetTarget%20Location (Math|Vector|MakeVector (.x _returnvalue) (.y _returnvalue) (- (.z (.WorldLocation (Class|PlayerController|DeprojectScreenPositiontoWorld _asplayer_controller (.x Location) (.y Location)))) (+ (.z (Variables|/Script/Engine.SceneComponent|GetRelativeLocation (Variables|Default|GetCableEnd))) -2e+01))))
    (Variables|Default|SetIsMoving true))
  (:Released
    (goto _label))
  (:Moved
    (goto _label)))

(fn ConstructionScript)

(fn UpdateLocation
  (params (Component :type Scene%20Component%20Object%20Reference) (Speed :type Float%20%28single-precision%29) (Target%20Location :type Vector))
  (bind _returnvalue (Transformation|GetWorldLocation Component))
  (if (Variables|Default|GetIsMoving)
    (if (Math|Float|NearlyEqual(Float) (.Z (Math|Vector|BreakVector Target%20Location)) (.Z (Math|Vector|BreakVector _returnvalue)) 2.0)
      (Variables|Default|SetIsMoving false)
      (else
        (Variables|Default|SetIsMoving true)
        (Transformation|AddWorldOffset Component (Math|Vector|MakeVector 0.0 0.0 (* (Math|Float|SelectFloat 1.0 -1.0 (> (.z (- Target%20Location _returnvalue)) 0.0)) Speed (Utilities|Time|GetWorldDeltaSeconds))) false false)))))