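; Player actor for the "Segura" tap minigame, where Giovanna holds up the Forninho by keeping a balance value in range.
; Progress drains each tick at a speed set by difficulty and round time, while taps raise it.
; Progress drives the Barra position, actor pitch and sprite; leaving either end reports a loss to GM_Segura and tweens a bouncing fall.
; IsGreen exposes the bar's state, and Dance freezes play to show the dance visual.
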(event EventBeginPlay
  (bind _barra (Variables|Default|GetBarra))
  (bind _asgm_segura (Utilities|Casting|CastToGM_Segura (Game|GetGameMode)))
  (bind _asbp_guido_instance (Utilities|Casting|CastToBP_GuidoInstance (Game|GetGameInstance)))
  (Variables|Default|SetFalling%20speed (* (Variables|/Game/Base/BP_GuidoInstance.BP_GuidoInstance_C|GetDificulty _asbp_guido_instance) (/ 2.0 (Variables|/Game/Base/GM_MicroGame.GM_MicroGame_C|GetMax%20Time _asgm_segura))))
  (bind _output_get (Variables|Default|SetProgress 0.5))
  (if (Utilities|IsValid _barra)
    (Default|SetPosition _barra _output_get)
    (if (> (Math|Random|RandomFloat) 0.994)
      (Rendering|SetVisibility (Variables|Default|GetFoG) true false))))

(event Collision|EventActorBeginOverlap
  (params (OtherActor :type Actor%20Object%20Reference)))

(event EventTick
  (params (DeltaSeconds :type Float%20%28single-precision%29))
  (bind _output_get (Variables|Default|SetProgress (+ (Variables|Default|GetProgress) (* DeltaSeconds (Variables|Default|GetFalling%20speed) -1.0))))
  (if (< _output_get 0.0)
    (bind _asgm_segura (Utilities|Casting|CastToGM_Segura (Game|GetGameMode)))
    (Default|Lost _asgm_segura)
    (Actor|Tick|SetActorTickEnabled false)
    (Variables|Default|SetLost true)
    (Default|TranslationTween (Variables|Default|GetBP_TweenComponent) "/Game/Curves/OutBounce.OutBounce" self "0, 0, 0" "0,100.000000,-500.000000" "NewEnumerator1" 1.0 "1,1,1" 0.0 3e+01)
    (Transformation|SetRelativeLocation (Variables|Default|GetForninho) "0, 0,210.000000" false false)
    (Components|Activation|Activate (Variables|Default|GetS_Giovana) false)
    (else
      (CallFunction|UpdatePosition _output_get))))

(event Input|TouchEvents|InputTouch
  (params (Location :type Vector) (FingerIndex :type ETouchIndex%20Enum))
  (:Pressed
    (if (not (Variables|Default|GetLost))
      (bind _output_get (Variables|Default|SetProgress (+ (Variables|Default|GetProgress) (Variables|Default|GetUpClick))))
      (Development|PrintString (Utilities|String|ToString(Float) _output_get))
      (if (> _output_get 1.0)
        (bind _asgm_segura (Utilities|Casting|CastToGM_Segura (Game|GetGameMode)))
        (Default|Lost _asgm_segura)
        (Actor|Tick|SetActorTickEnabled false)
        (Variables|Default|SetLost true)
        (Default|SetPosition (Variables|Default|GetBarra) 1.0)
        (Default|TranslationTween (Variables|Default|GetBP_TweenComponent) "/Game/Curves/OutBounce.OutBounce" self "0, 0, 0" "0,100.000000,-500.000000" "NewEnumerator1" 1.0 "1,1,1" 0.0 3e+01)
        (Transformation|SetRelativeLocation (Variables|Default|GetForninho) "0, 0,210.000000" false false)
        (Components|Activation|Activate (Variables|Default|GetS_Giovana) false)
        (else
          (CallFunction|UpdatePosition _output_get))))))

(fn ConstructionScript)

(fn AddOffsetFloat
  (params (Variable :type Float%20%28single-precision%29%20%28by%20ref%29) (Offset :type Float%20%28single-precision%29))
  (return (+ Variable Offset)))

(fn UpdatePosition
  (params (Progress :type Float%20%28single-precision%29))
  (bind _barra (Variables|Default|GetBarra))
  (if (Utilities|IsValid _barra)
    (Default|SetPosition _barra Progress))
  (Transformation|SetActorRotation (Math|Rotator|MakeRotator 0.0 (- (* Progress -6e+01) -3e+01) 0.0))
  (if (<= Progress 0.3)
    (Rendering|Components|Sprite|SetSprite (Variables|Default|GetGiovanna) "/Game/Sprites/SP_Forninho_Segurando1.SP_Forninho_Segurando1")
    (else
      (Rendering|Components|Sprite|SetSprite (Variables|Default|GetGiovanna) "/Game/Sprites/SP_Forninho_Segurando2.SP_Forninho_Segurando2"))))

(fn IsGreen
  (return (Default|IsGreen (Variables|Default|GetBarra))))

(fn Dance
  (Rendering|SetVisibility (Variables|Default|GetPaperSprite) false false)
  (Rendering|SetVisibility (Variables|Default|GetGiovanna) false false)
  (Rendering|SetVisibility (Variables|Default|GetDanca) true false)
  (Actor|Tick|SetActorTickEnabled false)
  (Variables|Default|SetLost true)
  (Utilities|FlowControl|DoOnce false))