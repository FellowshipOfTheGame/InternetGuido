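; BP_Cage is a cage actor that makes a punchy entrance when it spawns, with a sound and a camera shake at its location.
; On BeginPlay it starts at zero scale, then BPTweenComponent scales it in along a curve while tweening the active face sprite's color.
; A UseVariation flag picks between Face and AlternateFace, setting visibility in the construction script and choosing the sprite to tween.
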(event EventBeginPlay
  (Audio|PlaySound2D "/Game/Sound/SC_Anime_Punch.SC_Anime_Punch")
  (Camera|PlayWorldCameraShake "/Game/Base/ShortCameraShake.ShortCameraShake_C" (Transformation|GetActorLocation) 0.0 1e+03 0.0 true)
  (Transformation|SetActorScale3D "0, 0, 0")
  (Default|ScaleTween (Variables|Default|GetBP_TweenComponent) "/Game/Base/Curves/CageScaleIn.CageScaleIn" self 0.5 "1.000000,1.000000,1.000000" "1.000000,1.000000,1.000000" 0.0 3e+01)
  (Default|SpriteColorTween (Variables|Default|GetBP_TweenComponent) "/Game/Base/Curves/LinearColor.LinearColor" (CallFunction|GetActiveFace) 0.2 "1,1,1" 3.0 0.0 3e+01))

(fn ConstructionScript
  (bind _usevariation (Variables|Default|GetUseVariation))
  (Rendering|SetVisibility (Variables|Default|GetAlternateFace) _usevariation false)
  (Rendering|SetVisibility (Variables|Default|GetFace) (not _usevariation) false))

(fn GetActiveFace
  (return (select (Variables|Default|GetUseVariation) (Variables|Default|GetAlternateFace) (Variables|Default|GetFace))))