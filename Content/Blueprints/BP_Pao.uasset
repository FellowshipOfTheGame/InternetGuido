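; BP_Pao is a sprite actor that wins the game once no clouds are left overlapping it.
; On each end overlap, it scans its Box for remaining BP_Cloud actors and calls Win on the GM_Pa game mode if none is found.
; Its construction script reads the difficulty from BP_GuidoInstance and sets the sprite's opacity, making it fainter at later difficulty options.
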(event EventBeginPlay)

(event Collision|EventActorBeginOverlap
  (params (OtherActor :type Actor%20Object%20Reference)))

(event EventTick
  (params (DeltaSeconds :type Float%20%28single-precision%29)))

(event Collision|EventActorEndOverlap
  (params (OtherActor :type Actor%20Object%20Reference))
  (Variables|Default|SetFoundCloud false)
  (bind _array_element (Utilities|Array|ForEachLoopwithBreak (Collision|GetOverlappingActors (Variables|Default|GetBox) 0 :!class /Script/Engine.PrimitiveComponent) :!label _label)
    (:LoopBody
      (if (== (Utilities|GetClass _array_element) "/Game/Blueprints/BP_Cloud.BP_Cloud_C")
        (Variables|Default|SetFoundCloud true)
        (goto _label Break)))
    (:Completed
      (if (not (Variables|Default|GetFoundCloud))
        (bind _asgm_pa (Utilities|Casting|CastToGM_Pa (Game|GetGameMode)))
        (Default|Win _asgm_pa)))))

(fn ConstructionScript
  (bind _asbp_guido_instance (Utilities|Casting|CastToBP_GuidoInstance (Game|GetGameInstance)))
  (Sprite|SetSpriteColor (Variables|Default|GetPaperSprite) (Math|Color|MakeColor 1.0 1.0 1.0 (Utilities|Select :Index (Variables|/Game/Base/BP_GuidoInstance.BP_GuidoInstance_C|GetDificulty _asbp_guido_instance) :Option%200 1.0 :Option%201 0.9 :Option%202 0.7 :Option%203 0.5))))