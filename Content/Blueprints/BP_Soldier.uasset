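; Enemy soldier that creeps toward the player's ape while unwatched and ends the game on contact when advancing.
; An attention timer, shown on a spawned overhead progress bar, rises while the ape faces its side and falls otherwise.
; The timer's limits switch Tick states between standing, advancing and retreating, with bounce-tweened turns and toggled running/idle meshes.
; Overlapping the ape while advancing freezes the soldier, calls Lost on GM_Ape and shrinks the ape.
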(event Custom|AnimationParameters
  ;[1 1 1] AnimationPresents
  (Components|Timeline|SetPlayRate (Variables|Default|GetRunning) (/ (Variables|Default|GetSpeed) 35.0)))

(event Custom|Animation
  (bind _returnvalue (Utilities|Time|GetWorldDeltaSeconds))
  (bind _returnvalue_2 (Utilities|Time|GetWorldDeltaSeconds))
  (bind _legrotation (Variables|Animation|GetLegRotation))
  (bind _legjoinrotation (Variables|Animation|GetLegJoinRotation))
  (bind _llegjoint (Variables|Default|GetLLegJoint))
  (bind _rlegjoint (Variables|Default|GetRLegJoint))
  (bind _returnvalue_3 (* _legjoinrotation _returnvalue))
  (bind _returnvalue_4 (* _legrotation _returnvalue_2))
  ;[0.21 0 0.001422] UNUSED
  (switch int (Variables|Default|GetState)
    (:0
      (if (!= (Variables|Default|GetState) (Variables|Animation|GetPreviousAnimationStep))
        (Rendering|SetVisibility (Variables|Default|GetRunning) true false)
        (Rendering|SetVisibility (Variables|Default|GetBody) false true)))
    (:1
      (if (!= (Variables|Default|GetState) (Variables|Animation|GetPreviousAnimationStep)) :!label _label
        (Transformation|SetRelativeRotation (Variables|Default|GetLLeg) "80.000000, 0, 0" false false)
        (Transformation|SetRelativeRotation (Variables|Default|GetLLegJoint) "40.000000, 0, 0" false false)
        (Transformation|SetRelativeRotation (Variables|Default|GetRLeg) "-50.000000, 0, 0" false false)
        (Transformation|SetRelativeRotation (Variables|Default|GetRLegJoint) "-20.000000, 0, 0" false false)
        (Variables|Animation|SetPreviousAnimationStep (Variables|Default|GetState))
        (Variables|Animation|SetAnimationTimer 0.0)
        (Variables|Animation|SetAnimationStep 0)
        (else
          (CallFunction|RotationOffset (Variables|Default|GetLLeg) _returnvalue_4 (< (Variables|Animation|GetAnimationStep) 2))
          (CallFunction|RotationOffset (Variables|Default|GetRLeg) _returnvalue_4 (not (< (Variables|Animation|GetAnimationStep) 2)))
          (switch int (Variables|Animation|GetAnimationStep)
            (:0
              (CallFunction|RotationOffset _llegjoint _returnvalue_3 (== (Variables|Animation|GetAnimationStep) 1)))
            (:1
              (CallFunction|RotationOffset _llegjoint _returnvalue_3 (== (Variables|Animation|GetAnimationStep) 1)))
            (:2
              (CallFunction|RotationOffset _rlegjoint _returnvalue_3 (== (Variables|Animation|GetAnimationStep) 3)))
            (:3
              (CallFunction|RotationOffset _rlegjoint _returnvalue_3 (== (Variables|Animation|GetAnimationStep) 3))))
          (if (>= (+ (Variables|Animation|GetAnimationTimer) (Utilities|Time|GetWorldDeltaSeconds)) (Variables|Animation|GetMaxAnimation))
            (Variables|Animation|SetAnimationTimer 0.0)
            (bind _result (Math|Integer|IncrementInt (Variables|Animation|GetAnimationStep))
              (:%20%20
                (if (> _result 3)
                  (Variables|Animation|SetAnimationStep 0))))
            (else
              (Variables|Animation|SetAnimationTimer (+ (Variables|Animation|GetAnimationTimer) (Utilities|Time|GetWorldDeltaSeconds))))))))
    (:2
      (goto _label))))

(event EventDestroyed
  ;[1 1 1] Destroyed
  (Actor|Tick|SetActorTickEnabled false)
  (Actor|DestroyActor (Variables|Default|GetProgressBar)))

(event EventBeginPlay
  ;[1 1 1] Start
  (CallFunction|CalculateRightSide)
  (Variables|Default|SetSpeed 4e+01)
  (Transformation|SetWorldRotation (Variables|Default|GetRoot) (Math|Rotator|MakeRotator 0.0 0.0 (Math|Float|SelectFloat 0.0 1.8e+02 (Variables|Default|GetRightCorner))) false false)
  (Utilities|Casting|CastToBP_Ape (Game|Player|GetPlayerPawn 0))
  (Variables|Default|SetAtentionMax 1.0)
  (Variables|Default|SetAtententionTimer 0.0)
  (Variables|Default|SetState 1)
  (bind _returnvalue (Game|SpawnActorfromClass "/Game/Blueprints/BP_ProgressBar.BP_ProgressBar_C" (Math|Transform|MakeTransform (+ (Transformation|GetActorLocation) "0, 0,100.000000") "0, 0, 0" "2.000000,2.000000,2.000000") "Undefined" self 0))
  (bind _output_get (Variables|Default|SetProgressBar _returnvalue))
  (Class|Actor|AttachRootComponenttoActor _output_get self "None" "KeepWorldPosition" false)
  (CallFunction|AnimationParameters))

(event EventTick
  (params (DeltaSeconds :type Float%20%28single-precision%29))
  (if (not (Variables|Default|GetColided))
    (bind (_upper _down) (CallFunction|UpdateAtention))
    (switch int (Variables|Default|GetState)
      (:0
        (CallFunction|SwitchAnimation false)
        (if _upper
          (Variables|Default|SetState 2)
          (elif _down
            (Variables|Default|SetState 1)
            (CallFunction|Rotate))))
      (:1
        (CallFunction|UpdateLocation)
        (CallFunction|SwitchAnimation true)
        (if _upper
          (Variables|Default|SetState 2)
          (CallFunction|Rotate)
          (CallFunction|ResetAtention)))
      (:2
        (CallFunction|SwitchAnimation true)
        (CallFunction|UpdateLocation)
        (if _down
          (Variables|Default|SetState 0)
          (CallFunction|ResetAtention))))))

(event Collision|EventActorBeginOverlap
  (params (OtherActor :type Actor%20Object%20Reference))
  ;[1 1 1] Ape Colision
  (if (and (== OtherActor (Game|Player|GetPlayerPawn 0)) (== (Variables|Default|GetState) 1))
    (Actor|Tick|SetActorTickEnabled false)
    (Variables|Default|SetState 0)
    (Variables|Default|SetColided true)
    (Rendering|SetVisibility (Variables|Default|GetRunning) false false)
    (Rendering|SetVisibility (Variables|Default|GetBody) true true)
    (Development|PrintString "Hello")
    (bind _asgm_ape (Utilities|Casting|CastToGM_Ape (Game|GetGameMode)))
    (if (not (Variables|/Game/Base/GM_MicroGame.GM_MicroGame_C|GetIsGameLost _asgm_ape))
      (Default|Lost _asgm_ape)
      (bind _asbp_ape (Utilities|Casting|CastToBP_Ape OtherActor))
      (Default|Shrink _asbp_ape))))

(fn ConstructionScript
  (if (Variables|Default|GetUseVariant)
    _))

(fn UpdateLocation
  (Transformation|SetActorLocation (+ (* (Math|Vector|GetForwardVector (Variables|Default|GetDirection)) (* (Utilities|Time|GetWorldDeltaSeconds) (Variables|Default|GetSpeed))) (Transformation|GetActorLocation)) false false))

(fn Rotate
  (bind _returnvalue (Transformation|GetActorRotation))
  (Default|RotationTween (Variables|Default|GetBP_TweenComponent) "/Game/Curves/OutBounce.OutBounce" self _returnvalue (Math|Rotator|CombineRotators _returnvalue "0.000000,180.000000, 0") "NewEnumerator1" 1.0 "1, 1, 1" 0.0 3e+01 false))

(fn IsBeingSeen
  (bind _asbp_ape (Utilities|Casting|CastToBP_Ape (Game|Player|GetPlayerPawn 0))
    (:then
      (bind _output_get (Variables|Default|SetIsBeignSeen? (not (Class|KismetMathLibrary|XORBoolean (Variables|/Game/Blueprints/BP_Ape.BP_Ape_C|GetIsRight _asbp_ape) (Variables|Default|GetRightCorner))))))
    (:CastFailed
      _))
  (return _output_get))

(fn UpdateAtention
  (bind _asbp_ape (Utilities|Casting|CastToBP_Ape (Game|Player|GetPlayerPawn 0))
    (:then
      _)
    (:CastFailed
      _))
  (bind _output_get (Variables|Default|SetAtententionTimer (+ (Variables|Default|GetAtententionTimer) (* (Math|Integer|SelectInt 1 -1 (not (Class|KismetMathLibrary|XORBoolean (Variables|/Game/Blueprints/BP_Ape.BP_Ape_C|GetIsRight _asbp_ape) (Variables|Default|GetRightCorner)))) (Utilities|Time|GetWorldDeltaSeconds)))))
  (if (> _output_get (Variables|Default|GetAtentionMax))
    (LocalVariables|SetDownFlow false)
    (LocalVariables|SetUpperFlow true)
    (Variables|Default|SetAtententionTimer (Variables|Default|GetAtentionMax))
    (elif (<= _output_get 0.0)
      (LocalVariables|SetDownFlow true)
      (LocalVariables|SetUpperFlow false)
      (Variables|Default|SetAtententionTimer 0.0)
      (else
        (LocalVariables|SetDownFlow false)
        (LocalVariables|SetUpperFlow false))))
  (Default|SetScale (Variables|Default|GetProgressBar) (/ (Variables|Default|GetAtententionTimer) (Variables|Default|GetAtentionMax)))
  (return (LocalVariables|GetUpperFlow) (LocalVariables|GetDownFlow)))

(fn CalculateRightSide
  (bind _asbp_ape (Utilities|Casting|CastToBP_Ape (Game|Player|GetPlayerPawn 0)))
  (Variables|Default|SetRightCorner (>= (.x (- (Transformation|GetWorldLocation (Variables|Default|GetRoot)) (Transformation|GetWorldLocation (Variables|/Game/Blueprints/BP_Ape.BP_Ape_C|GetRoot _asbp_ape)))) 0.0)))

(fn ResetAtention
  (Variables|Default|SetAtententionTimer (Variables|Default|GetAtentionMax))
  (Default|SetScale (Variables|Default|GetProgressBar) (/ (Variables|Default|GetAtententionTimer) (Variables|Default|GetAtentionMax))))

(fn RotationOffset
  (params (Component :type Scene%20Component%20Object%20Reference) (RotationOffset :type Rotator) (Subtract :type Boolean))
  (Transformation|SetRelativeRotation Component (Math|Rotator|CombineRotators (Variables|/Script/Engine.SceneComponent|GetRelativeRotation Component) (* RotationOffset (Math|Integer|SelectInt -1 1 Subtract))) false false))

(fn SwitchAnimation
  (params (Running :type Boolean))
  (if (not (Variables|Default|GetColided))
    (Rendering|SetVisibility (Variables|Default|GetRunning) Running false)
    (Rendering|SetVisibility (Variables|Default|GetBody) (not Running) true)))