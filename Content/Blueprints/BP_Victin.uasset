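; BP_Victin is the sprite-based victim, which registers itself with BP_Assassin and reacts to spoon hits.
; BeginPlay derives walk and reaction timings from GM_Murder's MaxTime.
; Tick procedurally animates walking by moving the actor along Z and rotating arm parts, reversing whenever the walk timer expires.
; SpoonHit plays a scale tween on the ScaredSoldier curve while swapping head sprites in delayed steps.
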(event Custom|Spoon%20Hit
  (Default|ScaleTween (Variables|Default|GetBP_TweenComponent) "/Game/Base/Curves/ScaredSoldier.ScaredSoldier" self (* 2.0 (Variables|Default|GetDelayTime)) (Transformation|GetActorScale3D) "1, 1, 1" 0.0 3e+01)
  (Rendering|Components|Sprite|SetSprite (Variables|Default|GetHead) "/Game/Sprites/SP_VictinHead2.SP_VictinHead2")
  (Utilities|FlowControl|Delay (Variables|Default|GetDelayTime))
  (Rendering|Components|Sprite|SetSprite (Variables|Default|GetHead) "/Game/Sprites/SP_VictinHead3.SP_VictinHead3")
  (Utilities|FlowControl|Delay (Variables|Default|GetDelayTime))
  (Rendering|Components|Sprite|SetSprite (Variables|Default|GetHead) "/Game/Sprites/SP_VictinHead1.SP_VictinHead1"))

(event EventBeginPlay
  (bind _asbp_assassin (Utilities|Casting|CastToBP_Assassin (Game|Player|GetPlayerPawn 0)))
  (Variables|/Game/Blueprints/BP_Assassin.BP_Assassin_C|SetVictin _asbp_assassin self)
  (bind _asgm_murder (Utilities|Casting|CastToGM_Murder (Game|GetGameMode)))
  (bind _output_get (Variables|Default|SetDefault%20Walking (* (Variables|/Game/Base/GM_MicroGame.GM_MicroGame_C|GetMax%20Time _asgm_murder) 0.1)))
  (Variables|Default|SetTransladation%20Velocity (Math|Vector|MakeVector 0.0 0.0 (/ 1e+02 _output_get)))
  (Variables|Default|SetDelayTime (* (Variables|/Game/Base/GM_MicroGame.GM_MicroGame_C|GetMax%20Time _asgm_murder) 0.03))
  (Variables|Default|SetRArmRot (Math|Rotator|MakeRotator 0.0 (/ -6e+01 (Variables|Default|GetDefault%20Walking)) 0.0))
  (Variables|Default|SetRForarmRot (Math|Rotator|MakeRotator 0.0 (/ -5e+01 (Variables|Default|GetDefault%20Walking)) 0.0)))

(event EventTick
  (params (DeltaSeconds :type Float%20%28single-precision%29))
  (bind _returnvalue (Utilities|Time|GetWorldDeltaSeconds))
  (Variables|Default|SetWalking%20Timer (- (Variables|Default|GetWalking%20Timer) DeltaSeconds))
  ;[1 1 1] Walking Animation
  (Transformation|AddActorWorldOffset (* (Variables|Default|GetTransladation%20Velocity) _returnvalue))
  (CallFunction|AddOffsetRotation (Variables|Default|GetRArm) (* (Variables|Default|GetRArmRot) _returnvalue))
  (CallFunction|AddOffsetRotation (Variables|Default|GetRForearm) (* (Variables|Default|GetRForarmRot) _returnvalue))
  (CallFunction|AddOffsetRotation (Variables|Default|GetLArm) (* (* (Variables|Default|GetRArmRot) _returnvalue) -1))
  (CallFunction|AddOffsetRotation (Variables|Default|GetLForearm) (* (Variables|Default|GetRForarmRot) _returnvalue))
  (if (<= (Variables|Default|GetWalking%20Timer) 0.0)
    (Variables|Default|SetTransladation%20Velocity (* (Variables|Default|GetTransladation%20Velocity) -1))
    (Variables|Default|SetRArmRot (* (Variables|Default|GetRArmRot) -1))
    (Variables|Default|SetRForarmRot (* (Variables|Default|GetRForarmRot) -1))
    (Variables|Default|SetWalking%20Timer (Variables|Default|GetDefault%20Walking))))

(fn ConstructionScript)

(fn AddOffsetRotation
  (params (Component :type Scene%20Component%20Object%20Reference) (Offset :type Rotator))
  (Transformation|SetRelativeRotation Component (Math|Rotator|CombineRotators Offset (Variables|/Script/Engine.SceneComponent|GetRelativeRotation Component)) false false))