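; BP_Leao is a touchable lion actor that can be tapped while its Clicado flag is true.
; A tap randomly either toggles the NCage component's visibility and activates CageCry, or toggles Jaula's visibility and activates LionRoar.
; Either outcome clears Clicado to block further taps, then calls DecreaseLions on the GM_Leao game mode.
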(event Custom|Foi%20Clicado
  ;[1 1 1] Clique
  (if (Math|Random|RandomBool)
    (Rendering|ToggleVisibility (Variables|Default|GetNCage) false)
    (Components|Activation|Activate (Variables|Default|GetCageCry) false)
    (else
      (Rendering|ToggleVisibility (Variables|Default|GetJaula) false)
      (Components|Activation|Activate (Variables|Default|GetLionRoar) false)))
  (Variables|Default|SetClicado false)
  (bind _asgm_leao (Utilities|Casting|CastToGM_Leao (Game|GetGameMode)))
  (Default|DecreaseLions _asgm_leao))

(event EventActorOnInputTouchBegin
  (params (FingerIndex :type ETouchIndex%20Enum :default "Touch1"))
  ;[1 1 1] Clique
  (if (Variables|Default|GetClicado)
    (CallFunction|FoiClicado)))

(fn ConstructionScript)