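; BP_Forninho is a moving actor that heads toward a Target and costs the player the game if it reaches a trigger box.
; On BeginPlay it derives Speed from target distance, Time and a random factor, and sets pitch from the X/Z offset.
; Tick sweeps it along the Head component's forward vector.
; Overlapping a TriggerBox calls Lost on GM_Forninho, then destroys the actor.
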(event Collision|EventActorBeginOverlap
  (params (OtherActor :type Actor%20Object%20Reference))
  (if (== (Utilities|GetClass OtherActor) "/Script/Engine.TriggerBox")
    (bind _asgm_forninho (Utilities|Casting|CastToGM_Forninho (Game|GetGameMode)))
    (Default|Lost _asgm_forninho)
    (Actor|DestroyActor)))

(event EventBeginPlay
  (bind _returnvalue (Transformation|GetActorLocation))
  (bind _target (Variables|Default|GetTarget))
  (bind _returnvalue_2 (- _target _returnvalue))
  (bind (_x _y _z) (Math|Vector|BreakVector _returnvalue_2))
  (Variables|Default|SetSpeed (/ (Math|Vector|VectorLength _returnvalue_2) (/ (Variables|Default|GetTime) (Math|Random|RandomFloatinRange 1.5 3.0))))
  (Transformation|SetActorRotation (Math|Rotator|MakeRotator 0.0 (Class|KismetMathLibrary|DegAtan2 _x _z) 0.0)))

(event EventTick
  (params (DeltaSeconds :type Float%20%28single-precision%29))
  (Transformation|AddActorWorldOffset (* (Math|Vector|GetForwardVector (Variables|Default|GetHead)) (* DeltaSeconds (Variables|Default|GetSpeed))) true))

(fn ConstructionScript)